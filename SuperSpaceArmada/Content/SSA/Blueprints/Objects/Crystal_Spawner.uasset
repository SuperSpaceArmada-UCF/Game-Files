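; Spawner actor that drops Crystals at random points within the game instance's BoundaryArea and runs timed Bonanza crate events.
; A looping timeline with random pauses spawns Crystals at fixed height.
; Tick, throttled by a random Delay, starts a Bonanza when the Player has no active event.
; Its timeline rains random Health or Energy crates via a short Delay, then clears the Player's event flags and attack/defense buffs.
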(event EventBeginPlay
  ;[1 1 1] Spawn Regular
  (Utilities|FlowControl|Delay 0.2)
  (bind _asssagame_instance (Utilities|Casting|CastToSSAGameInstance (Game|GetGameInstance)))
  (Utilities|IsValid (Variables|/Game/SSA/Blueprints/SSAGameInstance.SSAGameInstance_C|GetBoundary%20Area _asssagame_instance)
    (:Is%20Valid
      (Game|SpawnActorfromClass "/Game/SSA/Blueprints/Objects/Crystal.Crystal_C" (Math|Transform|MakeTransform (Math|Vector|MakeVector (.X (Math|Vector|BreakVector (Math|Random|RandomPointinBoundingBox (.Origin (Collision|GetActorBounds (Variables|/Game/SSA/Blueprints/SSAGameInstance.SSAGameInstance_C|GetBoundary%20Area _asssagame_instance) false)) (.BoxExtent (Collision|GetActorBounds (Variables|/Game/SSA/Blueprints/SSAGameInstance.SSAGameInstance_C|GetBoundary%20Area _asssagame_instance) false))))) (.Y (Math|Vector|BreakVector (Math|Random|RandomPointinBoundingBox (.Origin (Collision|GetActorBounds (Variables|/Game/SSA/Blueprints/SSAGameInstance.SSAGameInstance_C|GetBoundary%20Area _asssagame_instance) false)) (.BoxExtent (Collision|GetActorBounds (Variables|/Game/SSA/Blueprints/SSAGameInstance.SSAGameInstance_C|GetBoundary%20Area _asssagame_instance) false))))) 2.6e+02)) "Undefined" 0 0 :!label _label)
      (Timeline|Power%20Up%20Spawner PlayFromStart
        (:Finished
          (Utilities|FlowControl|Delay (Math|Random|RandomFloatinRange 1.0 5.0))
          (goto _label))))))

(event EventTick
  (params (DeltaSeconds :type Float%20%28single-precision%29))
  ;[1 1 1] Bonanza Event
  (Utilities|FlowControl|Delay (Math|Random|RandomFloatinRange 1e+01 2e+01))
  (bind _asplayer (Utilities|Casting|CastToPlayer (Game|GetPlayerCharacter 0)))
  (if (not (Variables|/Game/SSA/Blueprints/Player_Ships/Player.Player_C|GetEventOccuring _asplayer))
    (Variables|/Game/SSA/Blueprints/Player_Ships/Player.Player_C|SetBonanzaOccuring _asplayer true)
    (Variables|/Game/SSA/Blueprints/Player_Ships/Player.Player_C|SetEventOccuring _asplayer true)
    (Default|Bonanza _asplayer)
    (Utilities|FlowControl|Delay 5.0)
    (Timeline|Bonanza PlayFromStart
      (:Update
        (if (Variables|/Game/SSA/Blueprints/Player_Ships/Player.Player_C|GetEventOccuring _asplayer)
          (bind _asssagame_instance (Utilities|Casting|CastToSSAGameInstance (Game|GetGameInstance)))
          (Utilities|FlowControl|Delay 0.1)
          (if (== (Math|Random|RandomInteger 2) 0)
            (Game|SpawnActorfromClass "/Game/SSA/Blueprints/Objects/Health_Crate.Health_Crate_C" (Math|Transform|MakeTransform (Math|Vector|MakeVector (.X (Math|Vector|BreakVector (Math|Random|RandomPointinBoundingBox (.Origin (Collision|GetActorBounds (Variables|/Game/SSA/Blueprints/SSAGameInstance.SSAGameInstance_C|GetBoundary%20Area _asssagame_instance) false)) (.BoxExtent (Collision|GetActorBounds (Variables|/Game/SSA/Blueprints/SSAGameInstance.SSAGameInstance_C|GetBoundary%20Area _asssagame_instance) false))))) (.Y (Math|Vector|BreakVector (Math|Random|RandomPointinBoundingBox (.Origin (Collision|GetActorBounds (Variables|/Game/SSA/Blueprints/SSAGameInstance.SSAGameInstance_C|GetBoundary%20Area _asssagame_instance) false)) (.BoxExtent (Collision|GetActorBounds (Variables|/Game/SSA/Blueprints/SSAGameInstance.SSAGameInstance_C|GetBoundary%20Area _asssagame_instance) false))))) 2.6e+02)) "AdjustIfPossibleButAlwaysSpawn" 0 0)
            (else
              (Game|SpawnActorfromClass "/Game/SSA/Blueprints/Objects/Energy_Crate.Energy_Crate_C" (Math|Transform|MakeTransform (Math|Vector|MakeVector (.X (Math|Vector|BreakVector (Math|Random|RandomPointinBoundingBox (.Origin (Collision|GetActorBounds (Variables|/Game/SSA/Blueprints/SSAGameInstance.SSAGameInstance_C|GetBoundary%20Area _asssagame_instance) false)) (.BoxExtent (Collision|GetActorBounds (Variables|/Game/SSA/Blueprints/SSAGameInstance.SSAGameInstance_C|GetBoundary%20Area _asssagame_instance) false))))) (.Y (Math|Vector|BreakVector (Math|Random|RandomPointinBoundingBox (.Origin (Collision|GetActorBounds (Variables|/Game/SSA/Blueprints/SSAGameInstance.SSAGameInstance_C|GetBoundary%20Area _asssagame_instance) false)) (.BoxExtent (Collision|GetActorBounds (Variables|/Game/SSA/Blueprints/SSAGameInstance.SSAGameInstance_C|GetBoundary%20Area _asssagame_instance) false))))) 2.6e+02)) "AdjustIfPossibleButAlwaysSpawn" 0 0)))
          (else
            (Audio|Components|Audio|Stop (Variables|Default|GetBonanza))
            (bind _asplayer_2 (Utilities|Casting|CastToPlayer (Game|GetPlayerCharacter 0) :!label _label))
            (Variables|/Game/SSA/Blueprints/Player_Ships/Player.Player_C|SetEventOccuring _asplayer_2 false)
            (Variables|/Game/SSA/Blueprints/Player_Ships/Player.Player_C|SetBonanzaOccuring _asplayer_2 false)
            (Default|RemoveBonanza _asplayer_2)
            (Variables|/Game/SSA/Blueprints/Player_Ships/Player.Player_C|SetAtkBuff_Enemy _asplayer_2 0)
            (Variables|/Game/SSA/Blueprints/Player_Ships/Player.Player_C|SetAtkBuff_Player _asplayer_2 0)
            (Variables|/Game/SSA/Blueprints/Player_Ships/Player.Player_C|SetDefBuff_Player _asplayer_2 0)
            (Variables|/Game/SSA/Blueprints/Player_Ships/Player.Player_C|SetDefBuff_Enemy _asplayer_2 0))))
      (:Finished
        (goto _label)))))

(fn ConstructionScript)