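; Large asteroid debris actor that drifts along a random velocity and damages the player or enemy ships it hits, then destroys itself.
; Construction randomizes direction and rotation, and a timeline applies the direction through ProjectileMovement.
; Hits on six enemy classes route damage through the player's EnemyHPRemove.
; Tick destroys only small debris at zero HP, while SpawnSmall replaces the asteroid with three scaled-down, non-large pieces.
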(event Custom|Spawn%20Small
  (bind _returnvalue (Transformation|GetActorTransform))
  (bind _returnvalue_2 (Transformation|GetActorTransform))
  (bind _returnvalue_3 (Transformation|GetActorTransform))
  (bind (_location _rotation _scale) (Math|Transform|BreakTransform _returnvalue))
  (bind (_location_2 _rotation_2 _scale_2) (Math|Transform|BreakTransform _returnvalue_2))
  (bind (_location_3 _rotation_3 _scale_3) (Math|Transform|BreakTransform _returnvalue_3))
  ;[1 1 1] Spawn Small Asteroids
  (Utilities|FlowControl|Sequence
    (:then_0
      (bind _returnvalue_4 (Game|SpawnActorfromClass "/Game/SSA/Blueprints/Objects/Debris.Debris_C" (Math|Transform|MakeTransform (+ "250.000000,250.000000, 0" (Transformation|GetActorLocation)) _rotation_2 (/ _scale_2 2.25)) "Undefined" 0 0))
      (Variables|/Game/SSA/Blueprints/Objects/Debris.Debris_C|SetIsLarge _returnvalue_4 false))
    (:then_1
      (bind _returnvalue_5 (Game|SpawnActorfromClass "/Game/SSA/Blueprints/Objects/Debris.Debris_C" (Math|Transform|MakeTransform (+ "250.000000,-250.000000, 0" (Transformation|GetActorLocation)) _rotation_3 (/ _scale_3 2.25)) "Undefined" 0 0))
      (Variables|/Game/SSA/Blueprints/Objects/Debris.Debris_C|SetIsLarge _returnvalue_5 false))
    (:then_2
      (bind _returnvalue_6 (Game|SpawnActorfromClass "/Game/SSA/Blueprints/Objects/Debris.Debris_C" (Math|Transform|MakeTransform (+ "-220.000000,-180.000000, 0" (Transformation|GetActorLocation)) _rotation (/ _scale 2.25)) "Undefined" 0 0))
      (Variables|/Game/SSA/Blueprints/Objects/Debris.Debris_C|SetIsLarge _returnvalue_6 false))
    (:then_3
      (Actor|DestroyActor))))

(event EventBeginPlay
  ;[1 1 1] Generate Random Move To
  (Timeline|Timeline_0 Play
    (:Update
      (Game|Components|ProjectileMovement|SetVelocityinLocalSpace (Variables|Default|GetProjectileMovement) (Variables|Default|GetDirection)))))

(event Collision|EventHit
  (params (MyComp :type Primitive%20Component%20Object%20Reference) (Other :type Actor%20Object%20Reference) (OtherComp :type Primitive%20Component%20Object%20Reference) (bSelfMoved :type Boolean) (HitLocation :type Vector) (HitNormal :type Vector :default "0, 0, 0") (NormalImpulse :type Vector :default "0, 0, 0") (Hit :type Hit%20Result%20Structure%20%28by%20ref%29))
  ;[1 1 1] Collision function
  (CallFunction|DebrisCollisionFunction Other 0.2))

(event EventTick
  (params (DeltaSeconds :type Float%20%28single-precision%29))
  ;[1 1 1] CheckHP
  (if (<= (Variables|Default|GetDebris%20HP) 0.0)
    (if (not (Variables|Default|GetIsLarge))
      (Actor|DestroyActor))))

(fn ConstructionScript
  (bind _returnvalue (Math|Random|RandomFloatinRange -3e+01 3e+01))
  (bind _returnvalue_2 (Math|Random|RandomFloatinRange -4e+03 -5e+03))
  (Variables|Default|SetDirection (Math|Vector|MakeVector _returnvalue_2 _returnvalue_2 _returnvalue_2))
  (Variables|Default|SetRotation (Math|Rotator|MakeRotator _returnvalue _returnvalue _returnvalue)))

(fn DebrisCollisionFunction
  (params (Collider :type Actor%20Object%20Reference) (Damage%20Amount :type Float%20%28single-precision%29))
  (Development|PrintString (Utilities|GetDisplayName Collider))
  (bind _asplayer (Utilities|Casting|CastToPlayer Collider)
    (:then
      (Default|HPRemove _asplayer Damage%20Amount))
    (:CastFailed
      (Utilities|Casting|CastToEnemy_Human Collider
        (:then
          _)
        (:CastFailed
          (Utilities|Casting|CastToEnemy_Kratakos Collider
            (:then
              _)
            (:CastFailed
              (Utilities|Casting|CastToEnemy_Hive Collider
                (:then
                  _)
                (:CastFailed
                  (Utilities|Casting|CastToEnemy_Cephalon Collider
                    (:then
                      _)
                    (:CastFailed
                      (Utilities|Casting|CastToEnemy_Dragomir Collider
                        (:then
                          _)
                        (:CastFailed
                          (Utilities|Casting|CastToEnemy_Vultari Collider)))))))))))
      (bind _asplayer_2 (Utilities|Casting|CastToPlayer (Game|GetPlayerCharacter 0)))
      (Default|EnemyHPRemove _asplayer_2 Damage%20Amount)))
  (Actor|DestroyActor))