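; Power-up spawner actor whose graph is built to drop PP_Crate actors at random points within its own bounds, raised slightly on Z.
; After a random delay of a few seconds, random branches all spawn the same crate class and play the PowerUpSpawner timeline from the start.
; The timeline's Finished output loops back to the delay.
; No event feeds this chain, so it never runs as it stands.
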(fn ConstructionScript)