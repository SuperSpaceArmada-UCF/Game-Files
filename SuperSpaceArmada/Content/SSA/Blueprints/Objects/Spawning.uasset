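; Spawning is an actor that keeps dropping Health or Energy crates at random points within its own bounds.
; Tick feeds a random 3 to 9 second Delay, which acts as a repeating timer because it ignores calls while pending.
; A coin flip then picks the crate class, spawned unrotated at a random point in the actor's bounding box, raised by a fixed height.
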(event EventTick
  (params (DeltaSeconds :type Float%20%28single-precision%29))
  (bind (_origin _boxextent) (Collision|GetActorBounds false))
  (bind _returnvalue (Math|Random|RandomPointinBoundingBox _origin _boxextent))
  (bind _returnvalue_2 (+ _returnvalue "0, 0,110.000000"))
  (bind _returnvalue_3 (Math|Transform|MakeTransform _returnvalue_2))
  (Utilities|FlowControl|Delay (Math|Random|RandomFloatinRange 3.0 9.0))
  (if (== 1 (Math|Random|RandomInteger 2))
    (Game|SpawnActorfromClass "/Game/SSA/Blueprints/Objects/Health_Crate.Health_Crate_C" _returnvalue_3 "Undefined" 0 0)
    (else
      (Game|SpawnActorfromClass "/Game/SSA/Blueprints/Objects/Energy_Crate.Energy_Crate_C" _returnvalue_3 "Undefined" 0 0))))

(fn ConstructionScript)