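; PP_Crate is a production points pickup that plays a looping animation on its skeletal mesh.
; On hit, it passes the other actor to PPPickUp, which uses casts to identify who touched it.
; A Player gains a fixed increase to MaxPP and the crate is destroyed.
; Enemy_Human and Enemy_Kratakos also destroy the crate but gain nothing, while other actors leave it intact.
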(event Custom|PP%20Pick%20Up
  (params (Ref :type Actor%20Object%20Reference))
  (bind _asplayer (Utilities|Casting|CastToPlayer Ref)
    (:then
      (Variables|/Game/SSA/Blueprints/Player.Player_C|SetMaxPP _asplayer (+ (Variables|/Game/SSA/Blueprints/Player.Player_C|GetMaxPP _asplayer) 5.0)))
    (:CastFailed
      (Utilities|Casting|CastToEnemy_Human Ref
        (:then
          _)
        (:CastFailed
          (Utilities|Casting|CastToEnemy_Kratakos Ref)))))
  (Actor|DestroyActor))

(event Collision|EventHit
  (params (MyComp :type Primitive%20Component%20Object%20Reference) (Other :type Actor%20Object%20Reference) (OtherComp :type Primitive%20Component%20Object%20Reference) (bSelfMoved :type Boolean) (HitLocation :type Vector :default "0, 0, 0") (HitNormal :type Vector :default "0, 0, 0") (NormalImpulse :type Vector :default "0, 0, 0") (Hit :type Hit%20Result%20Structure%20%28by%20ref%29))
  (CallFunction|PPPickUp Other))

(event EventBeginPlay
  (Components|Animation|PlayAnimation (Variables|SkeletalMeshActor|GetSkeletalMeshComponent) "/Game/Geometry/Meshes/ProductionPoints_MeshwAnim_Anim.ProductionPoints_MeshwAnim_Anim" true))

(fn ConstructionScript)