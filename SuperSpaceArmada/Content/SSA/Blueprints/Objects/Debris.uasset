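; Debris actor that drifts across the level as a hazard, damaging the player or enemies it hits.
; A looping Delay from BeginPlay interpolates its location toward a fixed X and Z, re-rolling the target Y randomly each iteration.
; Hits remove player HP directly, while hits on Enemy_Human or Enemy_Kratakos route damage through the player's EnemyHPRemove.
; The debris destroys itself after dealing damage and ignores other colliders.
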(event EventBeginPlay
  ;[1 1 1] Generate Random Move To
  (Transformation|SetActorLocation (Math|Interpolation|VInterpTo (Transformation|GetActorLocation) (Math|Vector|MakeVector -1.71e+03 (Math|Random|RandomFloatinRange -1.95e+03 1.95e+03) 2.2e+02) (Utilities|Time|GetWorldDeltaSeconds) 0.5) false false :!label _label)
  (Utilities|FlowControl|Delay 0.01)
  (goto _label))

(event Collision|EventHit
  (params (MyComp :type Primitive%20Component%20Object%20Reference) (Other :type Actor%20Object%20Reference) (OtherComp :type Primitive%20Component%20Object%20Reference) (bSelfMoved :type Boolean) (HitLocation :type Vector :default "0, 0, 0") (HitNormal :type Vector :default "0, 0, 0") (NormalImpulse :type Vector :default "0, 0, 0") (Hit :type Hit%20Result%20Structure%20%28by%20ref%29))
  (CallFunction|DebrisCollisionFunc Other 0.2))

(fn ConstructionScript)

(fn DebrisCollisionFunc
  (params (Collider :type Actor%20Object%20Reference) (Damage%20Amount :type Float%20%28single-precision%29))
  (bind _asplayer (Utilities|Casting|CastToPlayer Collider)
    (:then
      (Default|HPRemove _asplayer Damage%20Amount))
    (:CastFailed
      (Utilities|Casting|CastToEnemy_Human Collider
        (:then
          _)
        (:CastFailed
          (Utilities|Casting|CastToEnemy_Kratakos Collider)))
      (bind _asplayer_2 (Utilities|Casting|CastToPlayer (Game|GetPlayerCharacter 0)))
      (Default|EnemyHPRemove _asplayer_2 Damage%20Amount)))
  (Actor|DestroyActor))