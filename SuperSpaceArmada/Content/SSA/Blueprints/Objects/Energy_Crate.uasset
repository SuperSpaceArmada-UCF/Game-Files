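; Energy crate pickup that restores energy to either the player or the enemy side when hit, then destroys itself.
; A player hit restores player energy, while a chain of casts identifies the enemy types.
; Enemy hits route through player character 0, which handles enemy energy restoration.
; During a Bonanza, the pickup also increments that side's attack buff, both stored on the Player.
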(event Collision|EventHit
  (params (MyComp :type Primitive%20Component%20Object%20Reference) (Other :type Actor%20Object%20Reference) (OtherComp :type Primitive%20Component%20Object%20Reference) (bSelfMoved :type Boolean) (HitLocation :type Vector :default "0, 0, 0") (HitNormal :type Vector :default "0, 0, 0") (NormalImpulse :type Vector :default "0, 0, 0") (Hit :type Hit%20Result%20Structure%20%28by%20ref%29))
  (CallFunction|EnergyPowerUp Other 0.25))

(fn ConstructionScript)

(fn EnergyPowerUp
  (params (Collider :type Actor%20Object%20Reference) (Energy%20Amount :type Float%20%28single-precision%29))
  (bind _asplayer (Utilities|Casting|CastToPlayer Collider)
    (:then
      (Default|EnergyRestore _asplayer Energy%20Amount)
      (if (Variables|/Game/SSA/Blueprints/Player_Ships/Player.Player_C|GetBonanzaOccuring _asplayer)
        (Variables|/Game/SSA/Blueprints/Player_Ships/Player.Player_C|SetAtkBuff_Player _asplayer (+ (Variables|/Game/SSA/Blueprints/Player_Ships/Player.Player_C|GetAtkBuff_Player _asplayer) 1))))
    (:CastFailed
      (Utilities|Casting|CastToEnemy_Human Collider
        (:then
          _)
        (:CastFailed
          (Utilities|Casting|CastToEnemy_Kratakos Collider
            (:then
              _)
            (:CastFailed
              (Utilities|Casting|CastToEnemy_Dragomir Collider
                (:then
                  _)
                (:CastFailed
                  (Utilities|Casting|CastToEnemy_Cephalon Collider
                    (:then
                      _)
                    (:CastFailed
                      (Utilities|Casting|CastToEnemy_Vultari Collider
                        (:then
                          _)
                        (:CastFailed
                          (Utilities|Casting|CastToEnemy_Hive Collider)))))))))))
      (bind _asplayer_2 (Utilities|Casting|CastToPlayer (Game|GetPlayerCharacter 0)))
      (Default|EnemyEnergyRestore _asplayer_2 Energy%20Amount)
      (if (Variables|/Game/SSA/Blueprints/Player_Ships/Player.Player_C|GetBonanzaOccuring _asplayer_2)
        (Variables|/Game/SSA/Blueprints/Player_Ships/Player.Player_C|SetAtkBuff_Enemy _asplayer_2 (+ (Variables|/Game/SSA/Blueprints/Player_Ships/Player.Player_C|GetAtkBuff_Enemy _asplayer_2) 1)))))
  (Actor|DestroyActor))