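; Game instance for SSA that spawns the player's chosen ship when level Blueprints call SpawnPlayerShip.
; A switch on Player1CurrentShip picks one of six faction pawn classes, spawns it at a random XY within a square around the origin at fixed height, and has player controller 0 possess it.
; Every valid branch then unpauses the game, while an out-of-range index only prints an error.
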(event Custom|Spawn%20Player%20Ship
  (bind _returnvalue (Math|Random|RandomFloatinRange -1e+03 1e+03))
  (bind _returnvalue_2 (Math|Random|RandomFloatinRange -1e+03 1e+03))
  (bind _returnvalue_3 (Math|Vector|MakeVector _returnvalue _returnvalue_2 266.0))
  (bind _returnvalue_4 (Math|Transform|MakeTransform _returnvalue_3 "0, 0, 0" "1.000000,1.000000,1.000000"))
  ;[1 1 1] Player Ship Spawner (Called from level BPs)
  (switch int (Variables|Default|GetPlayer%201%20Current%20Ship) ; SHIP TYPES:\n\n0 == Human\n1 == Kratakos\n2 == Dragomir\n3 == Vultaari\n4 == The Hive\n5 == Cephalon
    (:Default
      (Development|PrintString "SPAWN Array OUT OF BOUNDS" true true "(R=1.000000,G=0.000000,B=0.095176,A=1.000000)" 1e+01))
    (:0
      (bind _returnvalue_5 (Game|SpawnActorfromClass "/Game/SSA/Blueprints/Player_Ships/Player_Human.Player_Human_C" _returnvalue_4 "Undefined" 0 0))
      (Pawn|Possess (Game|GetPlayerController 0) _returnvalue_5)
      (Game|SetGamePaused false :!label _label))
    (:1
      (bind _returnvalue_6 (Game|SpawnActorfromClass "/Game/SSA/Blueprints/Player_Ships/Player_Kratakos.Player_Kratakos_C" _returnvalue_4 "Undefined" 0 0))
      (Pawn|Possess (Game|GetPlayerController 0) _returnvalue_6)
      (goto _label))
    (:2
      (bind _returnvalue_7 (Game|SpawnActorfromClass "/Game/SSA/Blueprints/Player_Ships/Player_Dragomir.Player_Dragomir_C" _returnvalue_4 "Undefined" 0 0))
      (Pawn|Possess (Game|GetPlayerController 0) _returnvalue_7)
      (goto _label))
    (:3
      (bind _returnvalue_8 (Game|SpawnActorfromClass "/Game/SSA/Blueprints/Player_Ships/Player_Vultaari.Player_Vultaari_C" _returnvalue_4 "Undefined" 0 0))
      (Pawn|Possess (Game|GetPlayerController 0) _returnvalue_8)
      (goto _label))
    (:4
      (bind _returnvalue_9 (Game|SpawnActorfromClass "/Game/SSA/Blueprints/Player_Ships/Player_Hive.Player_Hive_C" _returnvalue_4 "Undefined" 0 0))
      (Pawn|Possess (Game|GetPlayerController 0) _returnvalue_9)
      (goto _label))
    (:5
      (bind _returnvalue_10 (Game|SpawnActorfromClass "/Game/SSA/Blueprints/Player_Ships/Player_Cephalon.Player_Cephalon_C" _returnvalue_4 "Undefined" 0 0))
      (Pawn|Possess (Game|GetPlayerController 0) _returnvalue_10)
      (goto _label))))