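; Hive enemy ship that chases the player, launches drones or self-destructs, then triggers the next enemy spawn.
; Tick drives AIMoveTo with thruster effects, choosing an attack on arrival by a health threshold.
; Live health, energy and primary cooldown reside on the Player; the ship's own HP/energy variables are marked unused.
; A timeline applies distance-scaled damage outside the arena boundary, and BeginPlay registers the ship with GameInstance, HUD and Player.
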(event Custom|HP%20Restore
  (params (HP%20Plus :type Float%20%28single-precision%29))
  ;[1 1 1] (NOT BEING USED)AI HP/Energy
  (Variables|Default|SetAI_Health%20%28NOT%20USED%29 (+ HP%20Plus (Variables|Default|GetAI_Health%20%28NOT%20USED%29))))

(event Custom|HP%20Remove
  (params (HP%20Minus :type Float%20%28single-precision%29))
  ;[1 1 1] (NOT BEING USED)AI HP/Energy
  (Variables|Default|SetAI_Health%20%28NOT%20USED%29 (- HP%20Minus (Variables|Default|GetAI_Health%20%28NOT%20USED%29))))

(event Custom|Hive_Primary
  (bind _returnvalue (Transformation|GetActorRotation))
  ;[1 1 1] Hive Primary
  (bind _asplayer (Utilities|Casting|CastToPlayer (Game|Player|GetPlayerPawn 0)))
  (if (Variables|/Game/SSA/Blueprints/Player_Ships/Player.Player_C|GetPrimaryWeaponCD _asplayer)
    (if (>= (Variables|/Game/SSA/Blueprints/Player_Ships/Player.Player_C|GetEnemyEnergy _asplayer) (/ 1.0 (Variables|/Game/SSA/Blueprints/Player_Ships/Player.Player_C|GetEnemyMaxEnergy _asplayer)))
      (Variables|/Game/SSA/Blueprints/Player_Ships/Player.Player_C|SetPrimaryWeaponCD _asplayer false)
      (bind _returnvalue_2 (Audio|SpawnSound2D "/Game/SSA/Sound/Sound_Effects/Laser_Cue.Laser_Cue"))
      (Audio|Components|Audio|Play _returnvalue_2 0.0)
      (Game|SpawnActorfromClass "/Game/SSA/Blueprints/Weapons/Enemy_Hive_Drones.Enemy_Hive_Drones_C" (Math|Transform|MakeTransform (+ (* (Math|Vector|GetForwardVector _returnvalue) 4.2e+02) (Transformation|GetActorLocation)) _returnvalue) "Undefined" 0 0)
      (Default|EnemyEnergyRemove _asplayer (/ 1.5 (Variables|/Game/SSA/Blueprints/Player_Ships/Player.Player_C|GetEnemyMaxEnergy _asplayer)))
      (Utilities|FlowControl|Delay 1.0)
      (Variables|/Game/SSA/Blueprints/Player_Ships/Player.Player_C|SetPrimaryWeaponCD _asplayer true))))

(event Custom|Hive%20Secondary
  ;[1 1 1] Hive Secondary
  (bind _asplayer (Utilities|Casting|CastToPlayer (Game|Player|GetPlayerPawn 0)))
  (if (>= (Variables|/Game/SSA/Blueprints/Player_Ships/Player.Player_C|GetEnemyEnergy _asplayer) (/ 3.0 (Variables|/Game/SSA/Blueprints/Player_Ships/Player.Player_C|GetEnemyMaxEnergy _asplayer)))
    (CallFunction|EnergyRemove 1.0)
    (Pawn|Components|CharacterMovement|DisableMovement (Variables|Character|GetCharacterMovement))
    (Utilities|FlowControl|Delay 1.0)
    (Effects|SpawnEmitteratLocation "/Game/Effects/Particles/P_Hive_Explosion.P_Hive_Explosion" (Transformation|GetActorLocation))
    (Camera|PlayWorldCameraShake "/Game/Effects/ScreenShakeKratakosBoost.ScreenShakeKratakosBoost_C" "0, 0, 0" 0.0 1e+04)
    (Game|SpawnActorfromClass "/Game/SSA/Blueprints/Weapons/Hive_SelfDestruct.Hive_SelfDestruct_C" (Transformation|GetActorTransform) "Undefined" 0 0)
    (Rendering|SetActorHiddenInGame true)
    (Utilities|FlowControl|Delay 2.0)
    (Default|SpawnNextShipEnemy _asplayer)))

(event Custom|Energy%20Restore
  (params (Energy%20Plus :type Float%20%28single-precision%29))
  ;[1 1 1] (NOT BEING USED)AI HP/Energy
  (Variables|Default|SetAI_Energy%20%28NOT%20USED%29 (+ Energy%20Plus (Variables|Default|GetAI_Energy%20%28NOT%20USED%29))))

(event Custom|Energy%20Remove
  (params (Energy%20Minus :type Float%20%28single-precision%29))
  ;[1 1 1] (NOT BEING USED)AI HP/Energy
  (Variables|Default|SetAI_Energy%20%28NOT%20USED%29 (- Energy%20Minus (Variables|Default|GetAI_Energy%20%28NOT%20USED%29))))

(event EventBeginPlay
  ;[1 1 1] Set AI Variables and Ref
  (bind _asssagame_instance (Utilities|Casting|CastToSSAGameInstance (Game|GetGameInstance)))
  (Variables|/Game/SSA/Blueprints/SSAGameInstance.SSAGameInstance_C|SetEnemy%20Ref _asssagame_instance self)
  (bind _asplayer (Utilities|Casting|CastToPlayer (Game|GetPlayerCharacter 0)))
  (Variables|/Game/SSA/Blueprints/Player_Ships/Player.Player_C|SetEnemyMaxHP _asplayer 6.0)
  (Variables|/Game/SSA/Blueprints/Player_Ships/Player.Player_C|SetEnemyMaxEnergy _asplayer 1e+01)
  (Variables|/Game/SSA/Blueprints/Player_Ships/Player.Player_C|SetEnemyHealth _asplayer 1.0)
  (Variables|/Game/SSA/Blueprints/Player_Ships/Player.Player_C|SetEnemyEnergy _asplayer 1.0)
  ;[1 1 1] Set Enemy Ref inside HUD
  (bind _foundwidgets (Widget|GetAllWidgetsOfClass "/Game/SSA/Blueprints/Menues/HUD.HUD_C" false))
  (for _array_element _foundwidgets
    (bind _ashud (Utilities|Casting|CastToHUD _array_element))
    (Variables|/Game/SSA/Blueprints/Menues/HUD.HUD_C|SetEnemy%20Ref _ashud self)
    (bind _asplayer_2 (Utilities|Casting|CastToPlayer (Game|GetPlayerCharacter 0)))
    (Default|SetEnemyRef _asplayer_2)
    ;[1 1 1] Boundary Arena
    (Timeline|Boundary%20Tick Play
      (:Update
        (CallFunction|BoundaryDamage)))))

(event EventTick
  (params (DeltaSeconds :type Float%20%28single-precision%29))
  (bind _returnvalue (Game|GetPlayerController 0))
  (bind _mesh (Variables|Character|GetMesh))
  ;[1 1 1] AI Attempt
  (if (>= (Transformation|GetDistanceTo (Pawn|GetController) _returnvalue) (Variables|Default|GetMinDistance))
    (AI|AIMoveTo self "0, 0, 0" _returnvalue 3e+02 false
      (:then
        ;[1 1 1] Comment
        (Effects|SpawnEmitterAttached "/Game/Effects/Particles/P_Hive_Thruster.P_Hive_Thruster" _mesh (Class|SkinnedMeshComponent|GetBoneName _mesh 20) "0, 0, 0" "180.000000, 0,180.000000" "SnapToTargetIncludingScale"))
      (:OnSuccess
        ;[1 1 1] AI_Atk
        (Utilities|FlowControl|Delay 5.0)
        (if (>= (Variables|/Game/SSA/Blueprints/Player_Ships/Player.Player_C|GetEnemyHealth (stale EventBeginPlay _asplayer)) 3.0)
          (CallFunction|HivePrimary)
          (else
            (CallFunction|HiveSecondary)))))))

(fn ConstructionScript)

(fn BoundaryDamage
  ;[1 1 1] Boundary Tick
  (if (not (> (Utilities|Array|Length (Collision|GetOverlappingActors "/Game/SSA/Blueprints/HUD/Arena_Boundary.Arena_Boundary_C" :!class /Script/Engine.Actor)) 0))
    (bind _outactors (Actor|GetAllActorsOfClass "/Game/SSA/Blueprints/HUD/Arena_Boundary.Arena_Boundary_C"))
    (for _array_element _outactors
      (bind _asplayer (Utilities|Casting|CastToPlayer (Game|GetPlayerCharacter 0)))
      (Default|EnemyHPRemove _asplayer (* (/ (Math|Float|Absolute(Float) (- (Math|Vector|VectorLength (- (Transformation|GetActorLocation _array_element) (Transformation|GetActorLocation))) (Math|Vector|VectorLength (.BoxExtent (Collision|GetActorBounds _array_element false))))) 1.5e+03) 0.001)))))