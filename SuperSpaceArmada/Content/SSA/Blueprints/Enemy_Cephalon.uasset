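; Cephalon enemy for the arena fight, whose health and energy live on the Player; its own HP/energy variables are unused.
; BeginPlay registers it with the game instance and HUD, then starts a timeline applying distance-scaled damage outside the arena boundary.
; Tick chases the player with AIMoveTo and thruster effects, firing two energy-gated abilities on arrival.
; Primary spawns a power-wave trigger that drains energy; secondary teleports to a random point within the boundary.
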(event Custom|HP%20Restore
  (params (HP%20Plus :type Float%20%28single-precision%29))
  ;[1 1 1] (NOT BEING USED)AI HP/Energy
  (Variables|Default|SetAI_Health%20%28NOT%20USED%29 (+ HP%20Plus (Variables|Default|GetAI_Health%20%28NOT%20USED%29))))

(event Custom|HP%20Remove
  (params (HP%20Minus :type Float%20%28single-precision%29))
  ;[1 1 1] (NOT BEING USED)AI HP/Energy
  (Variables|Default|SetAI_Health%20%28NOT%20USED%29 (- HP%20Minus (Variables|Default|GetAI_Health%20%28NOT%20USED%29))))

(event Custom|Ceph%20Primary
  ;[1 1 1] Ceph Primary
  (bind _asplayer (Utilities|Casting|CastToPlayer (Game|Player|GetPlayerPawn 0)))
  (if (>= (Variables|/Game/SSA/Blueprints/Player_Ships/Player.Player_C|GetEnemyEnergy _asplayer) (/ 2.0 (Variables|/Game/SSA/Blueprints/Player_Ships/Player.Player_C|GetEnemyMaxEnergy _asplayer)))
    (bind _returnvalue (Effects|SpawnEmitterAttached "/Game/Effects/Particles/P_Gravity2.P_Gravity2" (Variables|Character|GetMesh) "None" "0,-8.000000,-20.000000" "0, 0, 0" "SnapToTargetIncludingScale"))
    (bind _returnvalue_2 (Game|SpawnActorfromClass "/Game/SSA/Blueprints/Weapons/Enemy_PowerWave_Trigger.Enemy_PowerWave_Trigger_C" (Transformation|GetActorTransform) "Undefined" 0 0))
    (AddComponent|AddChildActorComponent _returnvalue_2 false)
    (CallFunction|PowerWave)
    (else
      (Actor|DestroyActor _returnvalue_2)
      (Components|DestroyComponent _returnvalue)
      (CallFunction|PowerWave))))

(event Custom|Power%20Wave
  ;[1 1 1] Ceph Primary
  (if (>= (Variables|/Game/SSA/Blueprints/Player_Ships/Player.Player_C|GetEnemyEnergy (stale Custom|Ceph%20Primary _asplayer)) (/ 2.0 (Variables|/Game/SSA/Blueprints/Player_Ships/Player.Player_C|GetEnemyMaxEnergy (stale Custom|Ceph%20Primary _asplayer))))
    (Utilities|FlowControl|Delay 1.0)
    (Default|EnemyEnergyRemove (stale Custom|Ceph%20Primary _asplayer) (/ 2.0 (Variables|/Game/SSA/Blueprints/Player_Ships/Player.Player_C|GetEnemyMaxEnergy (stale Custom|Ceph%20Primary _asplayer))))
    (Actor|DestroyActor (stale Custom|Ceph%20Primary _returnvalue_2))
    (Components|DestroyComponent (stale Custom|Ceph%20Primary _returnvalue))
    (CallFunction|PowerWave)))

(event Custom|Ceph%20Secondary
  ;[1 1 1] Ceph Secondary
  (bind _asplayer (Utilities|Casting|CastToPlayer (Game|Player|GetPlayerPawn 0)))
  (if (Variables|/Game/SSA/Blueprints/Player_Ships/Player.Player_C|GetSecondaryWeaponCD _asplayer)
    (if (>= (Variables|/Game/SSA/Blueprints/Player_Ships/Player.Player_C|GetEnemyEnergy _asplayer) (/ 3.0 (Variables|/Game/SSA/Blueprints/Player_Ships/Player.Player_C|GetEnemyMaxEnergy _asplayer)))
      (Audio|PlaySound2D "/Game/SSA/Music/Sound_Effects/Cephalon/ceph_teleport.ceph_teleport")
      (Utilities|FlowControl|Delay 1.5)
      (Effects|SpawnEmitterAttached "/Game/Effects/Particles/P_Teleport.P_Teleport" (Variables|Character|GetMesh) "None" "0, 0, 0" "0,90.000000,90.000000" "SnapToTarget")
      (Variables|/Game/SSA/Blueprints/Player_Ships/Player.Player_C|SetSecondaryWeaponCD _asplayer false)
      (Variables|/Game/SSA/Blueprints/Player_Ships/Player.Player_C|SetEnemyEnergy _asplayer (- (Variables|/Game/SSA/Blueprints/Player_Ships/Player.Player_C|GetEnemyEnergy _asplayer) (/ 3.0 (Variables|/Game/SSA/Blueprints/Player_Ships/Player.Player_C|GetEnemyMaxEnergy _asplayer))))
      (CallFunction|TeleportCalc)
      (Transformation|Teleport (Math|Vector|MakeVector (.X (Math|Vector|BreakVector (Math|Random|RandomPointinBoundingBox (.Origin (Collision|GetActorBounds (Variables|/Game/SSA/Blueprints/SSAGameInstance.SSAGameInstance_C|GetBoundary%20Area (stale Custom|Teleport%20Calc _asssagame_instance)) false)) (.BoxExtent (Collision|GetActorBounds (Variables|/Game/SSA/Blueprints/SSAGameInstance.SSAGameInstance_C|GetBoundary%20Area (stale Custom|Teleport%20Calc _asssagame_instance)) false))))) (.Y (Math|Vector|BreakVector (Math|Random|RandomPointinBoundingBox (.Origin (Collision|GetActorBounds (Variables|/Game/SSA/Blueprints/SSAGameInstance.SSAGameInstance_C|GetBoundary%20Area (stale Custom|Teleport%20Calc _asssagame_instance)) false)) (.BoxExtent (Collision|GetActorBounds (Variables|/Game/SSA/Blueprints/SSAGameInstance.SSAGameInstance_C|GetBoundary%20Area (stale Custom|Teleport%20Calc _asssagame_instance)) false))))) (.Z (Math|Vector|BreakVector (Transformation|GetActorLocation)))) "0, 0, 0")
      (Variables|/Game/SSA/Blueprints/Player_Ships/Player.Player_C|SetSecondaryWeaponCD _asplayer true))))

(event Custom|Teleport%20Calc
  ;[1 1 1] Ceph Secondary
  (bind _asssagame_instance (Utilities|Casting|CastToSSAGameInstance (Game|GetGameInstance))))

(event Custom|Energy%20Restore
  (params (Energy%20Plus :type Float%20%28single-precision%29))
  ;[1 1 1] (NOT BEING USED)AI HP/Energy
  (Variables|Default|SetAI_Energy%20%28NOT%20USED%29 (+ Energy%20Plus (Variables|Default|GetAI_Energy%20%28NOT%20USED%29))))

(event Custom|Energy%20Remove
  (params (Energy%20Minus :type Float%20%28single-precision%29))
  ;[1 1 1] (NOT BEING USED)AI HP/Energy
  (Variables|Default|SetAI_Energy%20%28NOT%20USED%29 (- Energy%20Minus (Variables|Default|GetAI_Energy%20%28NOT%20USED%29))))

(event EventBeginPlay
  ;[1 1 1] Set AI Variables and Ref
  (bind _asssagame_instance (Utilities|Casting|CastToSSAGameInstance (Game|GetGameInstance)))
  (Variables|/Game/SSA/Blueprints/SSAGameInstance.SSAGameInstance_C|SetEnemy%20Ref _asssagame_instance self)
  (bind _asplayer (Utilities|Casting|CastToPlayer (Game|GetPlayerCharacter 0)))
  (Variables|/Game/SSA/Blueprints/Player_Ships/Player.Player_C|SetEnemyMaxHP _asplayer 14.0)
  (Variables|/Game/SSA/Blueprints/Player_Ships/Player.Player_C|SetEnemyMaxEnergy _asplayer 12.0)
  (Variables|/Game/SSA/Blueprints/Player_Ships/Player.Player_C|SetEnemyHealth _asplayer 1.0)
  (Variables|/Game/SSA/Blueprints/Player_Ships/Player.Player_C|SetEnemyEnergy _asplayer 1.0)
  ;[1 1 1] Set Enemy Ref inside HUD
  (bind _foundwidgets (Widget|GetAllWidgetsOfClass "/Game/SSA/Blueprints/Menues/HUD.HUD_C" false))
  (for _array_element _foundwidgets
    (bind _ashud (Utilities|Casting|CastToHUD _array_element))
    (Variables|/Game/SSA/Blueprints/Menues/HUD.HUD_C|SetEnemy%20Ref _ashud self)
    (bind _asplayer_2 (Utilities|Casting|CastToPlayer (Game|GetPlayerCharacter 0)))
    (Default|SetEnemyRef _asplayer_2)
    ;[1 1 1] Boundary Arena
    (Timeline|Boundary%20Tick Play
      (:Update
        (CallFunction|BoundaryDamage)))))

(event EventTick
  (params (DeltaSeconds :type Float%20%28single-precision%29))
  (bind _returnvalue (Game|GetPlayerController 0))
  (bind _mesh (Variables|Character|GetMesh))
  ;[1 1 1] AI Attempt
  (if (>= (Transformation|GetDistanceTo (Pawn|GetController) _returnvalue) (Variables|Default|GetMinDistance))
    (AI|AIMoveTo self "0, 0, 0" _returnvalue 2e+02 false
      (:then
        ;[1 1 1] Comment
        (Effects|SpawnEmitterAttached "/Game/Effects/Particles/P_PulseThruster.P_PulseThruster" _mesh (Class|SkinnedMeshComponent|GetBoneName _mesh 25) "0, 0, 0" "180.000000, 0,180.000000" "SnapToTargetIncludingScale")
        (Effects|SpawnEmitterAttached "/Game/Effects/Particles/P_PulseThruster.P_PulseThruster" _mesh (Class|SkinnedMeshComponent|GetBoneName _mesh 24) "0, 0, 0" "180.000000, 0,180.000000" "SnapToTargetIncludingScale"))
      (:OnSuccess
        ;[1 1 1] AI_Atk
        (Utilities|FlowControl|Delay 2.0)
        (CallFunction|CephPrimary)
        (Utilities|FlowControl|Delay 0.5)
        (CallFunction|CephSecondary)))))

(fn ConstructionScript)

(fn BoundaryDamage
  ;[1 1 1] Boundary Tick
  (if (not (> (Utilities|Array|Length (Collision|GetOverlappingActors "/Game/SSA/Blueprints/HUD/Arena_Boundary.Arena_Boundary_C" :!class /Script/Engine.Actor)) 0))
    (bind _outactors (Actor|GetAllActorsOfClass "/Game/SSA/Blueprints/HUD/Arena_Boundary.Arena_Boundary_C"))
    (for _array_element _outactors
      (bind _asplayer (Utilities|Casting|CastToPlayer (Game|GetPlayerCharacter 0)))
      (Default|EnemyHPRemove _asplayer (* (/ (Math|Float|Absolute(Float) (- (Math|Vector|VectorLength (- (Transformation|GetActorLocation _array_element) (Transformation|GetActorLocation))) (Math|Vector|VectorLength (.BoxExtent (Collision|GetActorBounds _array_element false))))) 1.5e+03) 0.001)))))