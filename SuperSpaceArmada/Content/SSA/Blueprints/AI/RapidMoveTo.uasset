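; RapidMoveTo is a Behavior Tree task that moves an EnemyAI1-controlled pawn to the actor held in its TargetToFollow blackboard key.
; On execute it casts the owner to EnemyAI1, caches that reference for later runs, and calls AIMoveTo with a very tight acceptance radius.
; It finishes successfully when the move succeeds; a failed move or cast never calls FinishExecute, leaving the task running.
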(event EventReceiveExecute
  (params (OwnerActor :type Actor%20Object%20Reference))
  (if (!= (Variables|Default|GetEnemyAIRef) 0)
    _
    (else
      (bind _asenemy_ai1 (Utilities|Casting|CastToEnemyAI1 OwnerActor))
      (Variables|Default|SetEnemyAIRef _asenemy_ai1)))
  (AI|AIMoveTo (Pawn|GetControlledPawn (Variables|Default|GetEnemyAIRef)) "0.000000,0.000000, 0" (AI|BehaviorTree|GetBlackboardValueasActor (Variables|Default|GetTarget%20to%20follow)) 1.0 false
    (:OnSuccess
      (AI|BehaviorTree|FinishExecute true))))