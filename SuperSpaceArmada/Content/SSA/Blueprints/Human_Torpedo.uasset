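; Human torpedo projectile that homes in on the enemy AI and damages it on contact.
; On spawn it reads the enemy reference from the HUD widget, sets an AI-tagged component as its homing target, and explodes after a short delay.
; Hitbox overlap with an AI-tagged actor reduces enemy HP through the Player, scaled by max HP, then spawns an explosion at the enemy and destroys the torpedo.
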(event OnComponentBeginOverlap(HitBox)
  (params (OtherActor :type Actor%20Object%20Reference) (OtherComp :type Primitive%20Component%20Object%20Reference) (OtherBodyIndex :type Integer) (bFromSweep :type Boolean) (SweepResult :type Hit%20Result%20Structure%20%28by%20ref%29))
  ;[1 1 1] Collison Enemy AI
  (if (Actor|ActorHasTag OtherActor "AI")
    (bind _asplayer (Utilities|Casting|CastToPlayer (Game|GetPlayerCharacter 0)))
    (Default|EnemyHPRemove _asplayer (/ 3.0 (Variables|/Game/SSA/Blueprints/Player.Player_C|GetEnemyMaxHP _asplayer)))
    (bind _foundwidgets (Widget|GetAllWidgetsOfClass "/Game/SSA/Blueprints/Menues/HUD.HUD_C" false))
    (for _array_element _foundwidgets
      (bind _ashud (Utilities|Casting|CastToHUD _array_element))
      (Effects|SpawnEmitteratLocation "/Game/Effects/Particles/P_Impact_Explosion.P_Impact_Explosion" (Transformation|GetActorLocation (Variables|/Game/SSA/Blueprints/Menues/HUD.HUD_C|GetEnemy%20Ref _ashud)))
      (Actor|DestroyActor))))

(event EventBeginPlay
  ;[1 1 1] Homing Mechanic to AI
  (bind _foundwidgets (Widget|GetAllWidgetsOfClass "/Game/SSA/Blueprints/Menues/HUD.HUD_C" false))
  (for _array_element _foundwidgets
    (bind _ashud (Utilities|Casting|CastToHUD _array_element))
    (for _array_element_2 (Actor|GetComponentsbyTag (Variables|/Game/SSA/Blueprints/Menues/HUD.HUD_C|GetEnemy%20Ref _ashud) "/Script/Engine.SceneComponent" "AI")
      _)
    (Variables|/Script/Engine.ProjectileMovementComponent|SetHomingTargetComponent (Variables|Components|GetProjectileMovement) _array_element_2)
    ;[1 1 1] Particle Effect
    (Utilities|FlowControl|Delay 1.0)
    (Effects|SpawnEmitteratLocation "/Game/Effects/Particles/P_Impact_Explosion.P_Impact_Explosion" (Transformation|GetActorLocation))
    (Actor|DestroyActor)))

(fn ConstructionScript)