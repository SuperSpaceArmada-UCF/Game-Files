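; Vultari enemy for an arena fight, registering itself with the game instance and HUD and keeping its live health and energy on the Player.
; Tick-driven AIMoveTo closes on the player or heads to an X-mirrored point with thruster effects.
; An energy check picks machine-gun fire or mines, capped by removing the oldest.
; A timeline drains health outside Arena_Boundary, scaled by distance; local HP/energy events are unused.
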(event Custom|HP%20Restore
  (params (HP%20Plus :type Float%20%28single-precision%29))
  ;[1 1 1] (NOT BEING USED)AI HP/Energy
  (Variables|Default|SetAI_Health%20%28NOT%20USED%29 (+ HP%20Plus (Variables|Default|GetAI_Health%20%28NOT%20USED%29))))

(event Custom|HP%20Remove
  (params (HP%20Minus :type Float%20%28single-precision%29))
  ;[1 1 1] (NOT BEING USED)AI HP/Energy
  (Variables|Default|SetAI_Health%20%28NOT%20USED%29 (- HP%20Minus (Variables|Default|GetAI_Health%20%28NOT%20USED%29))))

(event Custom|Vultaari%20Primary
  ;[1 1 1] Vultaari Primary
  (bind _asplayer (Utilities|Casting|CastToPlayer (Game|Player|GetPlayerPawn 0)))
  (if (>= (Variables|/Game/SSA/Blueprints/Player_Ships/Player.Player_C|GetEnemyEnergy _asplayer) 0.2)
    (Default|EnemyEnergyRemove _asplayer (/ 1.0 (Variables|/Game/SSA/Blueprints/Player_Ships/Player.Player_C|GetEnemyMaxEnergy _asplayer)))
    (bind _returnvalue (Game|SpawnActorfromClass "/Game/SSA/Blueprints/Weapons/Enemy_Vultaari_machine.Enemy_Vultaari_machine_C" (Transformation|GetActorTransform) "Undefined" 0 0))
    (AddComponent|AddChildActorComponent _returnvalue false)
    (if (Utilities|IsValid (stale _output_get))
      (if (not (Audio|Components|Audio|IsPlaying (stale _output_get)))
        (bind _returnvalue_2 (Audio|SpawnSound2D "/Game/SSA/Music/Sound_Effects/Vultaari/vulta_guns.vulta_guns" 0.4 :!label _label))
        (bind _output_get (Variables|/Game/SSA/Blueprints/Player_Ships/Player.Player_C|SetFirstAtk _asplayer _returnvalue_2))
        (Audio|Components|Audio|Play _output_get 0.0))
      (else
        (goto _label)))))

(event Custom|Vultaari%20Secondary
  ;[1 1 1] Vultaari Secondary
  (bind _asplayer (Utilities|Casting|CastToPlayer (Game|Player|GetPlayerPawn 0)))
  (if (>= (Variables|/Game/SSA/Blueprints/Player_Ships/Player.Player_C|GetEnemyEnergy _asplayer) (/ 2.0 (Variables|/Game/SSA/Blueprints/Player_Ships/Player.Player_C|GetEnemyMaxEnergy _asplayer)))
    (Default|EnemyEnergyRemove _asplayer (/ 2.0 (Variables|/Game/SSA/Blueprints/Player_Ships/Player.Player_C|GetEnemyMaxEnergy _asplayer)))
    (if (>= (Variables|Default|GetnMines) 12)
      (CallFunction|RemoveMine)
      (else
        (Variables|Default|SetnMines (+ (Variables|Default|GetnMines) 1))))
    (CallFunction|AddMine)))

(event Custom|Remove%20Mine
  (bind _enemyminesarray (Variables|Default|GetEnemyMinesArray))
  ;[1 1 1] Vultaari Secondary
  (Utilities|IsValid (Utilities|Array|Get(acopy) _enemyminesarray)
    (:Is%20Valid
      (Actor|DestroyActor _enemyminesarray))
    (:Is%20Not%20Valid
      _))
  (Utilities|Array|RemoveIndex _enemyminesarray))

(event Custom|Energy%20Restore
  (params (Energy%20Plus :type Float%20%28single-precision%29))
  ;[1 1 1] (NOT BEING USED)AI HP/Energy
  (Variables|Default|SetAI_Energy%20%28NOT%20USED%29 (+ Energy%20Plus (Variables|Default|GetAI_Energy%20%28NOT%20USED%29))))

(event Custom|Add%20Mine
  ;[1 1 1] Vultaari Secondary
  (bind _returnvalue (Game|SpawnActorfromClass "/Game/SSA/Blueprints/Weapons/Player_Mine.Player_Mine_C" (Transformation|GetActorTransform) "AlwaysSpawn" 0 0))
  (Utilities|Array|Add (Variables|Default|GetEnemyMinesArray) _returnvalue))

(event Custom|Energy%20Remove
  (params (Energy%20Minus :type Float%20%28single-precision%29))
  ;[1 1 1] (NOT BEING USED)AI HP/Energy
  (Variables|Default|SetAI_Energy%20%28NOT%20USED%29 (- Energy%20Minus (Variables|Default|GetAI_Energy%20%28NOT%20USED%29))))

(event EventTick
  (params (DeltaSeconds :type Float%20%28single-precision%29))
  (bind _self self)
  (bind _mesh (Variables|Character|GetMesh))
  (bind _player (Variables|Default|GetPlayer))
  (bind _returnvalue (Transformation|GetActorLocation _player))
  (bind (_x _y _z) (Math|Vector|BreakVector _returnvalue))
  ;[1 1 1] AI Attempt
  (CallFunction|GetRange)
  (if (>= (Variables|Default|GetDist) 4e+02)
    (AI|AIMoveTo _self "0, 0, 0" _player 8e+02 false
      (:then
        ;[1 1 1] AI_Atk
        (Utilities|FlowControl|Delay 0.5 :!label _label)
        (if (>= (Variables|/Game/SSA/Blueprints/Player_Ships/Player.Player_C|GetEnemyEnergy (stale EventBeginPlay _asplayer)) (/ (Variables|/Game/SSA/Blueprints/Player_Ships/Player.Player_C|GetEnemyMaxEnergy (stale EventBeginPlay _asplayer)) 2.0))
          (CallFunction|VultaariSecondary)
          (else
            (CallFunction|VultaariPrimary))))
      (:OnSuccess
        (if (<= (Variables|Default|GetDist) 4e+02) :!label _label_2
          (AI|AIMoveTo _self (Math|Vector|MakeVector (* _x -1.0) _y _z) 0 8e+02 false
            (:then
              ;[1 1 1] Comment
              (Effects|SpawnEmitterAttached "/Game/Effects/Particles/P_Vultaari_Thruster.P_Vultaari_Thruster" _mesh (Class|SkinnedMeshComponent|GetBoneName _mesh 9) "0, 0, 0" "180.000000, 0,180.000000" "SnapToTargetIncludingScale")
              (Effects|SpawnEmitterAttached "/Game/Effects/Particles/P_Vultaari_Thruster.P_Vultaari_Thruster" _mesh (Class|SkinnedMeshComponent|GetBoneName _mesh 4) "0, 0, 0" "180.000000, 0,180.000000" "SnapToTargetIncludingScale"))
            (:OnSuccess
              (goto _label))))))
    (else
      (goto _label_2))))

(event EventBeginPlay
  ;[1 1 1] Set AI Variables and Ref
  (bind _asssagame_instance (Utilities|Casting|CastToSSAGameInstance (Game|GetGameInstance)))
  (Variables|/Game/SSA/Blueprints/SSAGameInstance.SSAGameInstance_C|SetEnemy%20Ref _asssagame_instance self)
  (bind _asplayer (Utilities|Casting|CastToPlayer (Game|GetPlayerCharacter 0)))
  (Variables|/Game/SSA/Blueprints/Player_Ships/Player.Player_C|SetEnemyMaxHP _asplayer 1e+01)
  (Variables|/Game/SSA/Blueprints/Player_Ships/Player.Player_C|SetEnemyMaxEnergy _asplayer 1e+01)
  (Variables|/Game/SSA/Blueprints/Player_Ships/Player.Player_C|SetEnemyHealth _asplayer 1.0)
  (Variables|/Game/SSA/Blueprints/Player_Ships/Player.Player_C|SetEnemyEnergy _asplayer 1.0)
  ;[1 1 1] Set Enemy Ref inside HUD
  (bind _foundwidgets (Widget|GetAllWidgetsOfClass "/Game/SSA/Blueprints/Menues/HUD.HUD_C" false))
  (for _array_element _foundwidgets
    (bind _ashud (Utilities|Casting|CastToHUD _array_element))
    (Variables|/Game/SSA/Blueprints/Menues/HUD.HUD_C|SetEnemy%20Ref _ashud self)
    (bind _asplayer_2 (Utilities|Casting|CastToPlayer (Game|GetPlayerCharacter 0)))
    (Default|SetEnemyRef _asplayer_2)
    ;[1 1 1] Boundary Arena
    (Timeline|Boundary%20Tick Play
      (:Update
        (CallFunction|BoundaryDamage)))))

(fn ConstructionScript)

(fn BoundaryDamage
  ;[1 1 1] Boundary Tick
  (if (not (> (Utilities|Array|Length (Collision|GetOverlappingActors "/Game/SSA/Blueprints/HUD/Arena_Boundary.Arena_Boundary_C" :!class /Script/Engine.Actor)) 0))
    (bind _outactors (Actor|GetAllActorsOfClass "/Game/SSA/Blueprints/HUD/Arena_Boundary.Arena_Boundary_C"))
    (for _array_element _outactors
      (bind _asplayer (Utilities|Casting|CastToPlayer (Game|GetPlayerCharacter 0)))
      (Default|EnemyHPRemove _asplayer (* (/ (Math|Float|Absolute(Float) (- (Math|Vector|VectorLength (- (Transformation|GetActorLocation _array_element) (Transformation|GetActorLocation))) (Math|Vector|VectorLength (.BoxExtent (Collision|GetActorBounds _array_element false))))) 1.5e+03) 0.001)))))

(fn GetRange
  (bind _asplayer (Utilities|Casting|CastToPlayer (Game|Player|GetPlayerPawn 0))
    (:then
      (Variables|Default|SetPlayer _asplayer)
      (Variables|Default|SetDist (Transformation|GetDistanceTo self _asplayer)))
    (:CastFailed
      (Development|PrintText "Cast Failed!"))))