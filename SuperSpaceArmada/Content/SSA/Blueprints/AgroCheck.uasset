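; Behavior tree node for EnemyAI1 that checks each tick for a visible target to aggro on.
; Sphere-traces around the controlled pawn for desired object types, ignoring all EnemyBot actors, then line-traces on the Camera channel to each hit to confirm line of sight.
; A visible hit sets TargetToFollow and TargetLocation on the blackboard; a blocked one clears TargetToFollow, so the last hit processed decides the target.
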(event EventTick
  (params (OwnerActor :type Actor%20Object%20Reference) (DeltaSeconds :type Float%20%28single-precision%29))
  ;[1 1 1] Is EnemyAI Set?
  (if (!= (Variables|Default|GetEnemyAIRef) 0)
    _
    (else
      (bind _asenemy_ai1 (Utilities|Casting|CastToEnemyAI1 OwnerActor))
      (Variables|Default|SetEnemyAIRef _asenemy_ai1)))
  (bind _outactors (Actor|GetAllActorsOfClass "/Game/SSA/Blueprints/EnemyBot.EnemyBot_C"))
  (Variables|Default|SetMyLocation (Transformation|GetActorLocation (Pawn|GetControlledPawn (Variables|Default|GetEnemyAIRef))))
  (bind _outhits (Collision|MultiSphereTraceForObjects (Transformation|GetActorLocation (Pawn|GetControlledPawn (Variables|Default|GetEnemyAIRef))) (+ (Transformation|GetActorLocation (Pawn|GetControlledPawn (Variables|Default|GetEnemyAIRef))) "0, 0,15.000000") 0.0 (Variables|Default|GetDesiredObjectTypes) false _outactors "None"))
  (bind _array_element (Utilities|Array|ForEachLoopwithBreak _outhits)
    (:LoopBody
      (bind _outhit (Collision|LineTraceByChannel (Variables|Default|GetMyLocation) (Transformation|GetActorLocation (.HitActor (Collision|BreakHitResult _array_element))) "TraceTypeQuery2" false _outactors "None"))
      (if (== (.HitActor (Collision|BreakHitResult _outhit)) (.HitActor (Collision|BreakHitResult _array_element)))
        (Class|BTFunctionLibrary|SetBlackboardValueasObject (Variables|Default|GetTargetToFollow) (.HitActor (Collision|BreakHitResult _outhit)))
        (AI|BehaviorTree|SetBlackboardValueasVector (Variables|Default|GetTargetLocation) (Transformation|GetActorLocation (.HitActor (Collision|BreakHitResult _outhit))))
        (else
          (Class|BTFunctionLibrary|SetBlackboardValueasObject (Variables|Default|GetTargetToFollow)))))))