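; Player ship Blueprint for the Cephalon, which registers itself as the game instance's player and sets its health and energy stats.
; Holding primary fire spawns a gravity effect and power-wave trigger actor, while a delayed recursive PowerWave event loops the attack sound and drains energy.
; Secondary fire spends energy to teleport the ship to a random XY point inside the boundary area, gated by a cooldown.
; Acceleration spawns thruster particles on two mesh bones.
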(event Custom|Power%20Wave
  ;[1 1 1] Cephalon_Primary
  (if (Variables|Default|GetPressed)
    (if (Utilities|IsValid (Variables|Default|GetFirstAtk))
      (if (Audio|Components|Audio|IsPlaying (Variables|Default|GetFirstAtk))
        _
        (else
          (bind _returnvalue (Audio|SpawnSound2D "/Game/SSA/Music/Sound_Effects/Cephalon/ceph_attack.ceph_attack" :!label _label))
          (bind _output_get (Variables|Default|SetFirstAtk _returnvalue))
          (Audio|Components|Audio|Play _output_get 0.0)))
      (else
        (goto _label)))
    (if (>= (Variables|Default|GetEnergy) (/ 2.0 (Variables|Default|GetMaxEnergy)))
      (Utilities|FlowControl|Delay 1.0)
      (if (Variables|Default|GetPressed)
        (CallFunction|EnergyRemove (/ 2.0 (Variables|Default|GetMaxEnergy)))
        (CallFunction|PowerWave :!label _label_2))
      (else
        (Variables|Default|SetPressed false)
        (goto _label_2)))
    (else
      (Utilities|IsValid (stale Input|GamepadEvents|GamepadFaceButtonBottom _returnvalue_2)
        (:Is%20Valid
          (Actor|DestroyActor (stale Input|GamepadEvents|GamepadFaceButtonBottom _returnvalue_2)))
        (:Is%20Not%20Valid
          _))
      (Utilities|IsValid (Variables|Default|GetFirstAtk)
        (:Is%20Valid
          (Audio|Components|Audio|Stop (Variables|Default|GetFirstAtk)))))))

(event Custom|Teleport%20Calc
  ;[1 1 1] Cephalon_Secondary
  (bind _asssagame_instance (Utilities|Casting|CastToSSAGameInstance (Game|GetGameInstance))))

(event EventBeginPlay
  ;[1 1 1] Cephalon Construct
  (bind _asssagame_instance (Utilities|Casting|CastToSSAGameInstance (Game|GetGameInstance)))
  (Variables|/Game/SSA/Blueprints/SSAGameInstance.SSAGameInstance_C|SetPlayer%20Ref _asssagame_instance self)
  (Variables|Default|SetMaxHP 14.0)
  (Variables|Default|SetHealth 1.0)
  (Variables|Default|SetMaxEnergy 12.0)
  (Variables|Default|SetEnergy 1.0)
  (|CallParentFunction))

(event Input|GamepadEvents|GamepadFaceButtonRight
  (params (Key :type Key%20Structure :default "AnyKey"))
  ;[1 1 1] Cephalon_Secondary
  (:Pressed
    (if (Variables|Default|GetSecondaryWeaponCD)
      (if (>= (Variables|Default|GetEnergy) (/ 3.0 (Variables|Default|GetMaxEnergy)))
        (Audio|SpawnSound2D "/Game/SSA/Music/Sound_Effects/Cephalon/ceph_teleport.ceph_teleport")
        (Utilities|FlowControl|Delay 0.4)
        (Effects|SpawnEmitterAttached "/Game/Effects/Particles/P_Teleport.P_Teleport" (Variables|Character|GetMesh) "None" "0.000000, 0, 0" "0.000000,90.000000,90.000000" "SnapToTarget")
        (Variables|Default|SetSecondaryWeaponCD false)
        (Variables|Default|SetEnergy (- (Variables|Default|GetEnergy) (/ 3.0 (Variables|Default|GetMaxEnergy))))
        (CallFunction|TeleportCalc)
        (Transformation|Teleport (Math|Vector|MakeVector (.X (Math|Vector|BreakVector (Math|Random|RandomPointinBoundingBox (.Origin (Collision|GetActorBounds (Variables|/Game/SSA/Blueprints/SSAGameInstance.SSAGameInstance_C|GetBoundary%20Area (stale Custom|Teleport%20Calc _asssagame_instance)) false)) (.BoxExtent (Collision|GetActorBounds (Variables|/Game/SSA/Blueprints/SSAGameInstance.SSAGameInstance_C|GetBoundary%20Area (stale Custom|Teleport%20Calc _asssagame_instance)) false))))) (.Y (Math|Vector|BreakVector (Math|Random|RandomPointinBoundingBox (.Origin (Collision|GetActorBounds (Variables|/Game/SSA/Blueprints/SSAGameInstance.SSAGameInstance_C|GetBoundary%20Area (stale Custom|Teleport%20Calc _asssagame_instance)) false)) (.BoxExtent (Collision|GetActorBounds (Variables|/Game/SSA/Blueprints/SSAGameInstance.SSAGameInstance_C|GetBoundary%20Area (stale Custom|Teleport%20Calc _asssagame_instance)) false))))) (.Z (Math|Vector|BreakVector (Transformation|GetActorLocation)))) "0, 0, 0")
        (Utilities|FlowControl|Delay 1.0)
        (Variables|Default|SetSecondaryWeaponCD true)))))

(event Input|GamepadEvents|GamepadFaceButtonBottom
  (params (Key :type Key%20Structure :default "AnyKey"))
  (bind _firstatk (Variables|Default|GetFirstAtk))
  ;[1 1 1] Cephalon_Primary
  (:Pressed
    (if (>= (Variables|Default|GetEnergy) (/ 2.0 (Variables|Default|GetMaxEnergy)))
      (bind _returnvalue (Effects|SpawnEmitterAttached "/Game/Effects/Particles/P_Gravity2.P_Gravity2" (Variables|Character|GetMesh) "None" "0.000000,-8.000000,-20.000000" "0.000000,0.000000,0.000000" "SnapToTargetIncludingScale"))
      (Variables|Default|SetPressed true)
      (bind _returnvalue_2 (Game|SpawnActorfromClass "/Game/SSA/Blueprints/Weapons/Player_PowerWave_Trigger.Player_PowerWave_Trigger_C" (Transformation|GetActorTransform) "Undefined" 0 0))
      (AddComponent|AddChildActorComponent _returnvalue_2 false)
      (CallFunction|PowerWave)))
  (:Released
    (Variables|Default|SetPressed false)
    (Utilities|IsValid _firstatk
      (:Is%20Valid
        (Audio|Components|Audio|Stop _firstatk))
      (:Is%20Not%20Valid
        _))
    (Actor|DestroyActor _returnvalue_2)
    (Components|DestroyComponent _returnvalue)))

(event Input|MouseEvents|LeftMouseButton
  (params (Key :type Key%20Structure :default "AnyKey"))
  (bind _firstatk (Variables|Default|GetFirstAtk))
  ;[1 1 1] Cephalon_Primary
  (:Pressed
    (if (>= (Variables|Default|GetEnergy) (/ 2.0 (Variables|Default|GetMaxEnergy)))
      (bind _returnvalue (Effects|SpawnEmitterAttached "/Game/Effects/Particles/P_Gravity2.P_Gravity2" (Variables|Character|GetMesh) "None" "0.000000,-8.000000,-20.000000" "0.000000,0.000000,0.000000" "SnapToTargetIncludingScale"))
      (Variables|Default|SetPressed true)
      (bind _returnvalue_2 (Game|SpawnActorfromClass "/Game/SSA/Blueprints/Weapons/Player_PowerWave_Trigger.Player_PowerWave_Trigger_C" (Transformation|GetActorTransform) "Undefined" 0 0))
      (AddComponent|AddChildActorComponent _returnvalue_2 false)
      (CallFunction|PowerWave)))
  (:Released
    (Variables|Default|SetPressed false)
    (Utilities|IsValid _firstatk
      (:Is%20Valid
        (Audio|Components|Audio|Stop _firstatk))
      (:Is%20Not%20Valid
        _))
    (Actor|DestroyActor _returnvalue_2)
    (Components|DestroyComponent _returnvalue)))

(event Input|MouseEvents|RightMouseButton
  (params (Key :type Key%20Structure :default "AnyKey"))
  ;[1 1 1] Cephalon_Secondary
  (:Pressed
    (if (Variables|Default|GetSecondaryWeaponCD)
      (if (>= (Variables|Default|GetEnergy) (/ 3.0 (Variables|Default|GetMaxEnergy)))
        (Audio|SpawnSound2D "/Game/SSA/Music/Sound_Effects/Cephalon/ceph_teleport.ceph_teleport")
        (Utilities|FlowControl|Delay 0.4)
        (Effects|SpawnEmitterAttached "/Game/Effects/Particles/P_Teleport.P_Teleport" (Variables|Character|GetMesh) "None" "0.000000, 0, 0" "0.000000,90.000000,90.000000" "SnapToTarget")
        (Variables|Default|SetSecondaryWeaponCD false)
        (Variables|Default|SetEnergy (- (Variables|Default|GetEnergy) (/ 3.0 (Variables|Default|GetMaxEnergy))))
        (CallFunction|TeleportCalc)
        (Transformation|Teleport (Math|Vector|MakeVector (.X (Math|Vector|BreakVector (Math|Random|RandomPointinBoundingBox (.Origin (Collision|GetActorBounds (Variables|/Game/SSA/Blueprints/SSAGameInstance.SSAGameInstance_C|GetBoundary%20Area (stale Custom|Teleport%20Calc _asssagame_instance)) false)) (.BoxExtent (Collision|GetActorBounds (Variables|/Game/SSA/Blueprints/SSAGameInstance.SSAGameInstance_C|GetBoundary%20Area (stale Custom|Teleport%20Calc _asssagame_instance)) false))))) (.Y (Math|Vector|BreakVector (Math|Random|RandomPointinBoundingBox (.Origin (Collision|GetActorBounds (Variables|/Game/SSA/Blueprints/SSAGameInstance.SSAGameInstance_C|GetBoundary%20Area (stale Custom|Teleport%20Calc _asssagame_instance)) false)) (.BoxExtent (Collision|GetActorBounds (Variables|/Game/SSA/Blueprints/SSAGameInstance.SSAGameInstance_C|GetBoundary%20Area (stale Custom|Teleport%20Calc _asssagame_instance)) false))))) (.Z (Math|Vector|BreakVector (Transformation|GetActorLocation)))) "0, 0, 0")
        (Utilities|FlowControl|Delay 1.0)
        (Variables|Default|SetSecondaryWeaponCD true)))))

(event Input|KeyboardEvents|Acceleration
  (params (AxisValue :type Vector))
  (bind _mesh (Variables|Character|GetMesh))
  ;[1 1 1] Comment
  (Effects|SpawnEmitterAttached "/Game/Effects/Particles/P_PulseThruster.P_PulseThruster" _mesh (Class|SkinnedMeshComponent|GetBoneName _mesh 25) AxisValue "180.000000, 0,180.000000" "SnapToTargetIncludingScale")
  (Effects|SpawnEmitterAttached "/Game/Effects/Particles/P_PulseThruster.P_PulseThruster" _mesh (Class|SkinnedMeshComponent|GetBoneName _mesh 24) "0, 0, 0" "180.000000, 0,180.000000" "SnapToTargetIncludingScale"))

(fn ConstructionScript
  (|CallParentFunction))