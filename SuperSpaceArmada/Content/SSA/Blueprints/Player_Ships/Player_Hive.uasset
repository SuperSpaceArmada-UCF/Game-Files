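; Player_Hive is the Hive Construct player ship, which registers itself as PlayerRef on the SSA game instance and sets health and energy stats before running parent BeginPlay.
; Left mouse spawns a Hive_Drones actor ahead of the ship with a laser sound, gated by normalized energy and a delay-based cooldown.
; The Acceleration axis event spawns thruster emitters on three mesh bones on every call, without checking the axis value.
; The Hive_Secondary section is empty.
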(event EventBeginPlay
  ;[1 1 1] The Hive Construct
  (bind _asssagame_instance (Utilities|Casting|CastToSSAGameInstance (Game|GetGameInstance)))
  (Variables|/Game/SSA/Blueprints/SSAGameInstance.SSAGameInstance_C|SetPlayer%20Ref _asssagame_instance self)
  (Variables|Default|SetMaxHP 6.0)
  (Variables|Default|SetHealth 1.0)
  (Variables|Default|SetMaxEnergy 1e+01)
  (Variables|Default|SetEnergy 1.0)
  (|CallParentFunction))

(event Input|MouseEvents|RightMouseButton
  (params (Key :type Key%20Structure :default "AnyKey"))
  ;[1 1 1] Hive_Secondary
)

(event Input|MouseEvents|LeftMouseButton
  (params (Key :type Key%20Structure :default "AnyKey"))
  (bind _returnvalue (Transformation|GetActorRotation))
  ;[1 1 1] Hive_Primary
  (:Pressed
    (if (Variables|Default|GetPrimaryWeaponCD)
      (if (>= (Variables|Default|GetEnergy) (/ 1.0 (Variables|Default|GetMaxEnergy)))
        (Variables|Default|SetPrimaryWeaponCD false)
        (bind _returnvalue_2 (Audio|SpawnSound2D "/Game/SSA/Music/Sound_Effects/Laser_Cue.Laser_Cue"))
        (Audio|Components|Audio|Play _returnvalue_2 0.0)
        (Game|SpawnActorfromClass "/Game/SSA/Blueprints/Weapons/Hive_Drones.Hive_Drones_C" (Math|Transform|MakeTransform (+ (* (Math|Vector|GetForwardVector _returnvalue) 4.2e+02) (Transformation|GetActorLocation)) _returnvalue) "Undefined" 0 0)
        (CallFunction|EnergyRemove (/ 1.5 (Variables|Default|GetMaxEnergy)))
        (Utilities|FlowControl|Delay 1.0)
        (Variables|Default|SetPrimaryWeaponCD true)))))

(event Input|KeyboardEvents|Acceleration
  (params (AxisValue :type Vector))
  (bind _mesh (Variables|Character|GetMesh))
  ;[1 1 1] Comment
  (Effects|SpawnEmitterAttached "/Game/Effects/Particles/P_Thruster_Old.P_Thruster_Old" _mesh (Class|SkinnedMeshComponent|GetBoneName _mesh) AxisValue "180.000000, 0,180.000000" "SnapToTargetIncludingScale")
  (Effects|SpawnEmitterAttached "/Game/Effects/Particles/P_Thruster_Old.P_Thruster_Old" _mesh (Class|SkinnedMeshComponent|GetBoneName _mesh 6) AxisValue "180.000000, 0,180.000000" "SnapToTargetIncludingScale")
  (Effects|SpawnEmitterAttached "/Game/Effects/Particles/P_Thruster_Old.P_Thruster_Old" _mesh (Class|SkinnedMeshComponent|GetBoneName _mesh 2) AxisValue "180.000000, 0,180.000000" "SnapToTargetIncludingScale"))

(fn ConstructionScript
  (|CallParentFunction))