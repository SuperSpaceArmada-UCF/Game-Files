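; Kratakos player ship, a child Character Blueprint that sets its health and energy stats and registers itself as PlayerRef in the game instance.
; Left mouse fires a railgun projectile after a short charge effect, with sound and camera shake.
; Right mouse spends energy on a cooldown-gated ram lunge that spawns a ram trigger, launches the ship forward and makes it briefly immortal.
; The Acceleration event spawns thruster particles on three mesh bones.
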(event Custom|Ram_Copy
  ;[1 1 1] Kratakos_Secondary
  (bind _returnvalue (Game|SpawnActorfromClass "/Game/SSA/Blueprints/Weapons/Player_Ram_Trigger.Player_Ram_Trigger_C" (Transformation|GetActorTransform) "Undefined" 0 0))
  (AddComponent|AddChildActorComponent _returnvalue false)
  (Variables|Default|SetIsImmortal true)
  (Character|LaunchCharacter (* (Transformation|GetActorForwardVector) 1500) false false)
  (Utilities|FlowControl|Delay 0.5)
  (Utilities|IsValid _returnvalue
    (:Is%20Valid
      (Actor|DestroyActor _returnvalue)
      (Variables|Default|SetIsImmortal false))))

(event EventBeginPlay
  ;[1 1 1] Kratakos Construct
  (bind _asssagame_instance (Utilities|Casting|CastToSSAGameInstance (Game|GetGameInstance)))
  (Variables|/Game/SSA/Blueprints/SSAGameInstance.SSAGameInstance_C|SetPlayer%20Ref _asssagame_instance self)
  (Variables|Default|SetMaxHP 22.0)
  (Variables|Default|SetHealth 1.0)
  (Variables|Default|SetMaxEnergy 1e+01)
  (Variables|Default|SetEnergy 1.0)
  (|CallParentFunction))

(event Input|MouseEvents|RightMouseButton
  (params (Key :type Key%20Structure :default "AnyKey"))
  ;[1 1 1] Kratakos_Secondary
  (:Pressed
    (Camera|PlayWorldCameraShake "/Game/Effects/ScreenShakeKratakosBoost.ScreenShakeKratakosBoost_C" "0, 0, 0" 0.0 1e+04)
    (if (Variables|Default|GetSecondaryWeaponCD)
      (if (>= (Variables|Default|GetEnergy) 0.2)
        (Variables|Default|SetSecondaryWeaponCD false)
        (bind _returnvalue (Audio|SpawnSound2D "/Game/SSA/Music/Sound_Effects/Ram_Lunge_Cue.Ram_Lunge_Cue"))
        (Audio|Components|Audio|Play _returnvalue 0.0)
        (CallFunction|EnergyRemove (/ 2.0 (Variables|Default|GetMaxEnergy)))
        (CallFunction|RamCopy)
        (Utilities|FlowControl|Delay 1.0)
        (Variables|Default|SetSecondaryWeaponCD true)))))

(event Input|MouseEvents|LeftMouseButton
  (params (Key :type Key%20Structure :default "AnyKey"))
  (bind _returnvalue (Transformation|GetActorRotation))
  ;[1 1 1] Kratakos_Primary
  (:Pressed
    (Effects|SpawnEmitterAttached "/Game/Effects/Particles/P_Railgun_charge.P_Railgun_charge" (Variables|Character|GetMesh) "None" "50.000000, 0,50.000000" "0, 0, 0" "SnapToTargetIncludingScale")
    (Utilities|FlowControl|Delay 0.4)
    (bind _returnvalue_2 (Audio|SpawnSound2D "/Game/SSA/Music/Sound_Effects/Rail_Gun_Cue.Rail_Gun_Cue"))
    (Audio|Components|Audio|Play _returnvalue_2 0.0)
    (Game|SpawnActorfromClass "/Game/SSA/Blueprints/Weapons/Kratakos_Rail_Gun.Kratakos_Rail_Gun_C" (Math|Transform|MakeTransform (+ (* (Math|Vector|GetForwardVector _returnvalue) 4.2e+02) (Transformation|GetActorLocation)) _returnvalue) "Undefined" 0 (Game|GetInstigator))
    (Camera|PlayWorldCameraShake "/Game/Effects/ScreenShakeWeapons.ScreenShakeWeapons_C" "0, 0, 0" 0.0 1e+04)))

(event Input|KeyboardEvents|Acceleration
  (params (AxisValue :type Vector))
  (bind _mesh (Variables|Character|GetMesh))
  ;[1 1 1] Comment
  (Effects|SpawnEmitterAttached "/Game/Effects/Particles/P_Thruster_Old.P_Thruster_Old" _mesh (Class|SkinnedMeshComponent|GetBoneName _mesh) AxisValue "180.000000, 0,180.000000" "SnapToTargetIncludingScale")
  (Effects|SpawnEmitterAttached "/Game/Effects/Particles/P_Thruster_Old.P_Thruster_Old" _mesh (Class|SkinnedMeshComponent|GetBoneName _mesh 6) AxisValue "180.000000, 0,180.000000" "SnapToTargetIncludingScale")
  (Effects|SpawnEmitterAttached "/Game/Effects/Particles/P_Thruster_Old.P_Thruster_Old" _mesh (Class|SkinnedMeshComponent|GetBoneName _mesh 2) AxisValue "180.000000, 0,180.000000" "SnapToTargetIncludingScale"))

(fn ConstructionScript
  (|CallParentFunction))