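; Dragomir player ship, a child Blueprint that registers itself with the game instance and sets its own health and energy pools.
; Holding primary fire spawns a fire-breath actor with sound, while a recursive delayed event drains energy until release or depletion.
; Secondary fire spends energy to restore health with effects and sound, gated by a cooldown.
; Both attacks accept mouse or gamepad, and the acceleration event spawns thruster particles.
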(event Custom|Fire%20Breath
  ;[1 1 1] Dragomir_Primary
  (if (Variables|Default|GetPressed)
    (if (Utilities|IsValid (Variables|Default|GetSecondaryAtk))
      (if (Audio|Components|Audio|IsPlaying (Variables|Default|GetSecondaryAtk))
        _
        (else
          (bind _returnvalue (Audio|SpawnSound2D "/Game/SSA/Music/Sound_Effects/Dragomir/drago_flame.drago_flame" :!label _label))
          (bind _output_get (Variables|Default|SetSecondaryAtk _returnvalue))
          (Audio|Components|Audio|Play _output_get 0.0)))
      (else
        (goto _label)))
    (if (>= (Variables|Default|GetEnergy) (/ 3.0 (Variables|Default|GetMaxEnergy)))
      (Utilities|FlowControl|Delay 1.0)
      (if (Variables|Default|GetPressed)
        (CallFunction|EnergyRemove (/ 3.0 (Variables|Default|GetMaxEnergy)))
        (CallFunction|FireBreath :!label _label_2))
      (else
        (Variables|Default|SetPressed false)
        (goto _label_2)))
    (else
      (Utilities|IsValid (stale Input|GamepadEvents|GamepadFaceButtonBottom _returnvalue)
        (:Is%20Valid
          (Actor|DestroyActor (stale Input|GamepadEvents|GamepadFaceButtonBottom _returnvalue)))
        (:Is%20Not%20Valid
          _))
      (Utilities|IsValid (Variables|Default|GetSecondaryAtk)
        (:Is%20Valid
          (Audio|Components|Audio|Stop (Variables|Default|GetSecondaryAtk)))))))

(event EventBeginPlay
  ;[1 1 1] Dragomir Construct
  (bind _asssagame_instance (Utilities|Casting|CastToSSAGameInstance (Game|GetGameInstance)))
  (Variables|/Game/SSA/Blueprints/SSAGameInstance.SSAGameInstance_C|SetPlayer%20Ref _asssagame_instance self)
  (Variables|Default|SetMaxHP 16.0)
  (Variables|Default|SetHealth 1.0)
  (Variables|Default|SetMaxEnergy 13.0)
  (Variables|Default|SetEnergy 1.0)
  (|CallParentFunction))

(event Input|MouseEvents|RightMouseButton
  (params (Key :type Key%20Structure :default "AnyKey"))
  ;[1 1 1] Dragomir_Secondary
  (:Pressed
    (if (>= (Variables|Default|GetEnergy) (/ 4.0 (Variables|Default|GetMaxEnergy)))
      (if (Variables|Default|GetSecondaryWeaponCD)
        (Effects|SpawnEmitterAttached "/Game/Effects/Particles/P_Dragomir_Heal.P_Dragomir_Heal" (Variables|Character|GetMesh) "None")
        (Audio|SpawnSound2D "/Game/SSA/Music/Sound_Effects/Dragomir/drago_healing.drago_healing" 1.0)
        (Variables|Default|SetSecondaryWeaponCD false)
        (CallFunction|EnergyRemove (/ 4.0 (Variables|Default|GetMaxEnergy)))
        (CallFunction|HPRestore (/ 2.0 (Variables|Default|GetMaxHP)))
        (Utilities|FlowControl|Delay 2.0)
        (Variables|Default|SetSecondaryWeaponCD true)))))

(event Input|GamepadEvents|GamepadFaceButtonBottom
  (params (Key :type Key%20Structure :default "AnyKey"))
  (bind _secondaryatk (Variables|Default|GetSecondaryAtk))
  (:Pressed
    ;[1 1 1] Dragomir_Primary
    (if (>= (Variables|Default|GetEnergy) (/ 2.0 (Variables|Default|GetMaxEnergy)))
      (Variables|Default|SetPressed true)
      (CallFunction|EnergyRemove (/ 2.0 (Variables|Default|GetMaxEnergy)))
      (bind _returnvalue (Game|SpawnActorfromClass "/Game/SSA/Blueprints/Weapons/Player_FireBreath.Player_FireBreath_C" (Math|Transform|MakeTransform (.Location (Math|Transform|BreakTransform (Transformation|GetActorTransform))) "0, 0, 0" "3.000000,3.000000,3.000000") "Undefined" 0 0))
      (AddComponent|AddChildActorComponent _returnvalue false)
      (CallFunction|FireBreath)))
  (:Released
    (Variables|Default|SetPressed false)
    (Utilities|IsValid _secondaryatk
      (:Is%20Valid
        (Audio|Components|Audio|Stop _secondaryatk)
        (Utilities|IsValid _returnvalue
          (:Is%20Valid
            _)))
      (:Is%20Not%20Valid
        _))
    (Actor|DestroyActor _returnvalue)))

(event Input|GamepadEvents|GamepadFaceButtonRight
  (params (Key :type Key%20Structure :default "AnyKey"))
  ;[1 1 1] Dragomir_Secondary
  (:Pressed
    (if (>= (Variables|Default|GetEnergy) (/ 4.0 (Variables|Default|GetMaxEnergy)))
      (if (Variables|Default|GetSecondaryWeaponCD)
        (Effects|SpawnEmitterAttached "/Game/Effects/Particles/P_Dragomir_Heal.P_Dragomir_Heal" (Variables|Character|GetMesh) "None")
        (Audio|SpawnSound2D "/Game/SSA/Music/Sound_Effects/Dragomir/drago_healing.drago_healing" 1.0)
        (Variables|Default|SetSecondaryWeaponCD false)
        (CallFunction|EnergyRemove (/ 4.0 (Variables|Default|GetMaxEnergy)))
        (CallFunction|HPRestore (/ 2.0 (Variables|Default|GetMaxHP)))
        (Utilities|FlowControl|Delay 2.0)
        (Variables|Default|SetSecondaryWeaponCD true)))))

(event Input|MouseEvents|LeftMouseButton
  (params (Key :type Key%20Structure :default "AnyKey"))
  (bind _secondaryatk (Variables|Default|GetSecondaryAtk))
  ;[1 1 1] Dragomir_Primary
  (:Pressed
    (if (>= (Variables|Default|GetEnergy) (/ 2.0 (Variables|Default|GetMaxEnergy)))
      (Variables|Default|SetPressed true)
      (CallFunction|EnergyRemove (/ 2.0 (Variables|Default|GetMaxEnergy)))
      (bind _returnvalue (Game|SpawnActorfromClass "/Game/SSA/Blueprints/Weapons/Player_FireBreath.Player_FireBreath_C" (Math|Transform|MakeTransform (.Location (Math|Transform|BreakTransform (Transformation|GetActorTransform))) "0, 0, 0" "3.000000,3.000000,3.000000") "Undefined" 0 0))
      (AddComponent|AddChildActorComponent _returnvalue false)
      (CallFunction|FireBreath)))
  (:Released
    (Variables|Default|SetPressed false)
    (Utilities|IsValid _secondaryatk
      (:Is%20Valid
        (Audio|Components|Audio|Stop _secondaryatk)
        (Utilities|IsValid _returnvalue
          (:Is%20Valid
            _)))
      (:Is%20Not%20Valid
        _))
    (Actor|DestroyActor _returnvalue)))

(event Input|KeyboardEvents|Acceleration
  (params (AxisValue :type Vector))
  (bind _mesh (Variables|Character|GetMesh))
  ;[1 1 1] Comment
  (Effects|SpawnEmitterAttached "/Game/Effects/Particles/P_Thruster_Dragomir.P_Thruster_Dragomir" _mesh (Class|SkinnedMeshComponent|GetBoneName _mesh) AxisValue "180.000000, 0,180.000000" "SnapToTargetIncludingScale"))

(fn ConstructionScript
  (|CallParentFunction))