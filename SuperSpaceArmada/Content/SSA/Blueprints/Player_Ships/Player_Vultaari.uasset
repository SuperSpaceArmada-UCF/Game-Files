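; Player-controlled Vultaari ship that sets its health and energy stats and registers as PlayerRef in the game instance.
; Primary fire spends energy to spawn a Vultaari_machine and plays a phaser sound, avoiding overlapping playback.
; Secondary fire spends energy to drop mines, tracked in a capped array that destroys the oldest at the limit.
; Both attacks accept mouse or gamepad input, and the Acceleration event attaches thruster emitters to two mesh bones.
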(event Custom|Add%20Mine
  ;[1 1 1] Vultaari_Secondary
  (bind _returnvalue (Game|SpawnActorfromClass "/Game/SSA/Blueprints/Weapons/Player_Mine.Player_Mine_C" (Transformation|GetActorTransform) "AlwaysSpawn" 0 0))
  (Utilities|Array|Add (Variables|Default|GetMines%20Array) _returnvalue))

(event Custom|Remove%20Mine
  (bind _mines_array (Variables|Default|GetMines%20Array))
  (bind _item (Utilities|Array|Get(acopy) _mines_array))
  ;[1 1 1] Vultaari_Secondary
  (Utilities|IsValid _item
    (:Is%20Valid
      (Actor|DestroyActor _item))
    (:Is%20Not%20Valid
      _))
  (Utilities|Array|RemoveIndex (Variables|Default|GetMines%20Array)))

(event EventBeginPlay
  ;[1 1 1] Vultaari Construct
  (bind _asssagame_instance (Utilities|Casting|CastToSSAGameInstance (Game|GetGameInstance)))
  (Variables|/Game/SSA/Blueprints/SSAGameInstance.SSAGameInstance_C|SetPlayer%20Ref _asssagame_instance self)
  (Variables|Default|SetMaxHP 1e+01)
  (Variables|Default|SetHealth 1.0)
  (Variables|Default|SetMaxEnergy 1e+01)
  (Variables|Default|SetEnergy 1.0)
  (|CallParentFunction))

(event Input|MouseEvents|RightMouseButton
  (params (Key :type Key%20Structure :default "AnyKey"))
  ;[1 1 1] Vultaari_Secondary
  (:Pressed
    (if (>= (Variables|Default|GetEnergy) (/ 2.0 (Variables|Default|GetMaxEnergy)))
      (CallFunction|EnergyRemove (/ 2.0 (Variables|Default|GetMaxEnergy)))
      (if (>= (Variables|Default|GetnMines) 12)
        (CallFunction|RemoveMine)
        (else
          (Variables|Default|SetnMines (+ (Variables|Default|GetnMines) 1))))
      (CallFunction|AddMine))))

(event Input|GamepadEvents|GamepadFaceButtonBottom
  (params (Key :type Key%20Structure :default "AnyKey"))
  (:Pressed
    ;[1 1 1] Vultaari_Primary
    (if (>= (Variables|Default|GetEnergy) 0.2)
      (CallFunction|EnergyRemove (/ 1.0 (Variables|Default|GetMaxEnergy)))
      (bind _returnvalue (Game|SpawnActorfromClass "/Game/SSA/Blueprints/Weapons/Vultaari_machine.Vultaari_machine_C" (Transformation|GetActorTransform) "Undefined" 0 0))
      (AddComponent|AddChildActorComponent _returnvalue false)
      (if (Utilities|IsValid (Variables|Default|GetFirstAtk))
        (if (not (Audio|Components|Audio|IsPlaying (Variables|Default|GetFirstAtk)))
          (bind _returnvalue_2 (Audio|SpawnSound2D "/Game/SSA/Sound/Sound_Effects/Phasers.Phasers" :!label _label))
          (bind _output_get (Variables|Default|SetFirstAtk _returnvalue_2))
          (Audio|Components|Audio|Play _output_get 0.0))
        (else
          (goto _label))))))

(event Input|GamepadEvents|GamepadFaceButtonRight
  (params (Key :type Key%20Structure :default "AnyKey"))
  (:Pressed
    ;[1 1 1] Vultaari_Secondary
    (if (>= (Variables|Default|GetEnergy) (/ 2.0 (Variables|Default|GetMaxEnergy)))
      (CallFunction|EnergyRemove (/ 2.0 (Variables|Default|GetMaxEnergy)))
      (if (>= (Variables|Default|GetnMines) 12)
        (CallFunction|RemoveMine)
        (else
          (Variables|Default|SetnMines (+ (Variables|Default|GetnMines) 1))))
      (CallFunction|AddMine))))

(event Input|MouseEvents|LeftMouseButton
  (params (Key :type Key%20Structure :default "AnyKey"))
  ;[1 1 1] Vultaari_Primary
  (:Pressed
    (if (>= (Variables|Default|GetEnergy) 0.2)
      (CallFunction|EnergyRemove (/ 1.0 (Variables|Default|GetMaxEnergy)))
      (bind _returnvalue (Game|SpawnActorfromClass "/Game/SSA/Blueprints/Weapons/Vultaari_machine.Vultaari_machine_C" (Transformation|GetActorTransform) "Undefined" 0 0))
      (AddComponent|AddChildActorComponent _returnvalue false)
      (if (Utilities|IsValid (Variables|Default|GetFirstAtk))
        (if (not (Audio|Components|Audio|IsPlaying (Variables|Default|GetFirstAtk)))
          (bind _returnvalue_2 (Audio|SpawnSound2D "/Game/SSA/Sound/Sound_Effects/Phasers.Phasers" :!label _label))
          (bind _output_get (Variables|Default|SetFirstAtk _returnvalue_2))
          (Audio|Components|Audio|Play _output_get 0.0))
        (else
          (goto _label))))))

(event Input|KeyboardEvents|Acceleration
  (params (AxisValue :type Vector))
  (bind _mesh (Variables|Character|GetMesh))
  ;[1 1 1] Comment
  (Effects|SpawnEmitterAttached "/Game/Effects/Particles/P_Vultaari_Thruster.P_Vultaari_Thruster" _mesh (Class|SkinnedMeshComponent|GetBoneName _mesh 9) AxisValue "180.000000, 0,180.000000" "SnapToTargetIncludingScale")
  (Effects|SpawnEmitterAttached "/Game/Effects/Particles/P_Vultaari_Thruster.P_Vultaari_Thruster" _mesh (Class|SkinnedMeshComponent|GetBoneName _mesh 4) AxisValue "180.000000, 0,180.000000" "SnapToTargetIncludingScale"))

(fn ConstructionScript
  (|CallParentFunction))