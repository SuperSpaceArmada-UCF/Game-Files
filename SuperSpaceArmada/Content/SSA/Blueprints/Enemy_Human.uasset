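; Human enemy AI that pursues the player controller and fires torpedoes in the arena, with its own health and energy.
; Tick issues the move order and, through a one-second Delay, spawns a Human_Torpedo ahead of it.
; BeginPlay registers it with HUD widgets and starts a timeline applying distance-scaled damage outside Arena_Boundary.
; HPRemove and EnergyRemove subtract the current value from the amount, reversing the usual order.
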(event Custom|HP%20Restore
  (params (HP%20Plus :type Float%20%28single-precision%29))
  ;[1 1 1] AI HP/Energy
  (Variables|Default|SetAI_Health (+ HP%20Plus (Variables|Default|GetAI_Health))))

(event Custom|HP%20Remove
  (params (HP%20Minus :type Float%20%28single-precision%29))
  ;[1 1 1] AI HP/Energy
  (Variables|Default|SetAI_Health (- HP%20Minus (Variables|Default|GetAI_Health))))

(event Custom|Energy%20Restore
  (params (Energy%20Plus :type Float%20%28single-precision%29))
  ;[1 1 1] AI HP/Energy
  (Variables|Default|SetAI_Energy (+ Energy%20Plus (Variables|Default|GetAI_Energy))))

(event Custom|Energy%20Remove
  (params (Energy%20Minus :type Float%20%28single-precision%29))
  ;[1 1 1] AI HP/Energy
  (Variables|Default|SetAI_Energy (- Energy%20Minus (Variables|Default|GetAI_Energy))))

(event EventBeginPlay
  ;[1 1 1] Set Enemy Ref inside HUD
  (bind _foundwidgets (Widget|GetAllWidgetsOfClass "/Game/SSA/Blueprints/Menues/HUD.HUD_C" false))
  (for _array_element _foundwidgets
    (bind _ashud (Utilities|Casting|CastToHUD _array_element))
    (Variables|/Game/SSA/Blueprints/Menues/HUD.HUD_C|SetEnemy%20Ref _ashud self)
    ;[1 1 1] Boundary Arena
    (Timeline|Boundary%20Tick Play
      (:Update
        (CallFunction|BoundaryDamage)))))

(event EventTick
  (params (DeltaSeconds :type Float%20%28single-precision%29))
  (bind _returnvalue (Transformation|GetActorRotation))
  ;[1 1 1] AI Movement
  (AI|Navigation|SimpleMovetoActor (Pawn|GetController) (Game|GetPlayerController 0))
  ;[1 1 1] AI Attack
  (Utilities|FlowControl|Delay 1.0)
  (Game|SpawnActorfromClass "/Game/SSA/Blueprints/Human_Torpedo.Human_Torpedo_C" (Math|Transform|MakeTransform (+ (* (Math|Vector|GetForwardVector _returnvalue) 4.2e+02) (Transformation|GetActorLocation)) _returnvalue) "Undefined" 0 (Game|GetInstigator)))

(fn ConstructionScript)

(fn BoundaryDamage
  ;[1 1 1] Boundary Tick
  (if (not (> (Utilities|Array|Length (Collision|GetOverlappingActors "/Game/SSA/Blueprints/HUD/Arena_Boundary.Arena_Boundary_C" :!class /Script/Engine.Actor)) 0))
    (bind _outactors (Actor|GetAllActorsOfClass "/Game/SSA/Blueprints/HUD/Arena_Boundary.Arena_Boundary_C"))
    (for _array_element _outactors
      (CallFunction|HPRemove (* (/ (Math|Float|Absolute(Float) (- (Math|Vector|VectorLength (- (Transformation|GetActorLocation _array_element) (Transformation|GetActorLocation))) (Math|Vector|VectorLength (.BoxExtent (Collision|GetActorBounds _array_element false))))) 1.5e+03) 0.001)))))