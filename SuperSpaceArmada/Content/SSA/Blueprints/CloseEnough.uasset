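; CloseEnough is a Behavior Tree decorator that tests the distance between an EnemyAI1-controlled pawn and its follow target.
; It casts the owner to EnemyAI1, stores that reference, and measures from the controlled pawn to the TargetToFollow blackboard actor.
; The check passes when that distance is at least zero, so the threshold as set never rejects a measured distance.
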(fn PerformConditionCheck
  (params (OwnerActor :type Actor%20Object%20Reference))
  (bind _asenemy_ai1 (Utilities|Casting|CastToEnemyAI1 OwnerActor))
  (Variables|Default|SetEnemyAIRef _asenemy_ai1)
  (return (>= (Math|Vector|VectorLength (- (Transformation|GetActorLocation (AI|BehaviorTree|GetBlackboardValueasActor (Variables|Default|GetTarget%20to%20Follow))) (Transformation|GetActorLocation (Pawn|GetControlledPawn (Variables|Default|GetEnemyAIRef))))) 0.0)))