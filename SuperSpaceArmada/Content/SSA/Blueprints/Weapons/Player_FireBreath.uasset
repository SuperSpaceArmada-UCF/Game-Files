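; Player fire breath weapon actor that follows the player's location every tick and damages enemies tagged "AI".
; Its static mesh overlap removes enemy HP on entry and sets a flag that is cleared on exit.
; While flagged, a Delay inside Tick throttles repeated smaller damage.
; Damage goes through the Player's EnemyHPRemove as a fraction of EnemyMaxHP, so the overlapped actor is never damaged directly.
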(event OnComponentBeginOverlap(StaticMeshComponent)
  (params (OtherActor :type Actor%20Object%20Reference) (OtherComp :type Primitive%20Component%20Object%20Reference) (OtherBodyIndex :type Integer) (bFromSweep :type Boolean) (SweepResult :type Hit%20Result%20Structure%20%28by%20ref%29))
  ;[1 1 1] Begin/End overlap
  (if (Actor|ActorHasTag OtherActor "AI")
    (Variables|Default|SetAI true)
    (bind _asplayer (Utilities|Casting|CastToPlayer (Game|GetPlayerCharacter 0)))
    (Default|EnemyHPRemove _asplayer (/ 1.0 (Variables|/Game/SSA/Blueprints/Player_Ships/Player.Player_C|GetEnemyMaxHP _asplayer)))))

(event OnComponentEndOverlap(StaticMeshComponent)
  (params (OtherActor :type Actor%20Object%20Reference) (OtherComp :type Primitive%20Component%20Object%20Reference) (OtherBodyIndex :type Integer))
  ;[1 1 1] Begin/End overlap
  (if (Actor|ActorHasTag OtherActor "AI")
    (Variables|Default|SetAI false)))

(event EventTick
  (params (DeltaSeconds :type Float%20%28single-precision%29))
  ;[1 1 1] Follow Player
  (Transformation|SetActorLocation (Transformation|GetActorLocation (Game|GetPlayerCharacter 0)) false false)
  ;[1 1 1] Damage Tick
  (if (Variables|Default|GetAI)
    (Utilities|FlowControl|Delay 0.1)
    (bind _asplayer (Utilities|Casting|CastToPlayer (Game|GetPlayerCharacter 0)))
    (Default|EnemyHPRemove _asplayer (/ 0.6 (Variables|/Game/SSA/Blueprints/Player_Ships/Player.Player_C|GetEnemyMaxHP _asplayer)))))

(fn ConstructionScript)