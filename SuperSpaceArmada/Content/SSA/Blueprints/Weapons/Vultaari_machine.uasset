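; Vultaari machine weapon projectile that deals fixed damage to debris, the player or AI on Hitbox overlap, or explodes after a two-second lifetime.
; Actor tags select the target: debris loses raw HP, while player and enemy health drop by damage divided by max HP.
; Enemy health lives on the Player character, and AI hits use the HUD widget's EnemyRef to place the impact effect before destroying the projectile.
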(event OnComponentBeginOverlap(Hitbox)
  (params (OtherActor :type Actor%20Object%20Reference) (OtherComp :type Primitive%20Component%20Object%20Reference) (OtherBodyIndex :type Integer) (bFromSweep :type Boolean) (SweepResult :type Hit%20Result%20Structure%20%28by%20ref%29))
  (if (Actor|ActorHasTag OtherActor "Debris")
    (bind _asdebris (Utilities|Casting|CastToDebris OtherActor))
    (Variables|/Game/SSA/Blueprints/Objects/Debris.Debris_C|SetDebris%20HP _asdebris (- (Variables|/Game/SSA/Blueprints/Objects/Debris.Debris_C|GetDebris%20HP _asdebris) 3.0))
    (Effects|SpawnEmitteratLocation "/Game/Effects/Particles/P_Railgun_Impact.P_Railgun_Impact" (Transformation|GetActorLocation _asdebris))
    (Actor|DestroyActor)
    (elif (Actor|ActorHasTag OtherActor "Player")
      (bind _asplayer (Utilities|Casting|CastToPlayer (Game|GetPlayerCharacter 0)))
      (Variables|/Game/SSA/Blueprints/Player_Ships/Player.Player_C|SetHealth _asplayer (- (Variables|/Game/SSA/Blueprints/Player_Ships/Player.Player_C|GetHealth _asplayer) (/ 3.0 (Variables|/Game/SSA/Blueprints/Player_Ships/Player.Player_C|GetMaxHP _asplayer))))
      (Effects|SpawnEmitteratLocation "/Game/Effects/Particles/P_Railgun_Impact.P_Railgun_Impact" (Transformation|GetActorLocation _asplayer))
      (Actor|DestroyActor)
      (elif (Actor|ActorHasTag OtherActor "AI")
        (bind _asplayer_2 (Utilities|Casting|CastToPlayer (Game|GetPlayerCharacter 0)))
        (Variables|/Game/SSA/Blueprints/Player_Ships/Player.Player_C|SetEnemyHealth _asplayer_2 (- (Variables|/Game/SSA/Blueprints/Player_Ships/Player.Player_C|GetEnemyHealth _asplayer_2) (/ 3.0 (Variables|/Game/SSA/Blueprints/Player_Ships/Player.Player_C|GetEnemyMaxHP _asplayer_2))))
        (bind _foundwidgets (Widget|GetAllWidgetsOfClass "/Game/SSA/Blueprints/Menues/HUD.HUD_C" false))
        (for _array_element _foundwidgets
          (bind _ashud (Utilities|Casting|CastToHUD _array_element))
          (Utilities|IsValid (Variables|/Game/SSA/Blueprints/Menues/HUD.HUD_C|GetEnemy%20Ref _ashud)
            (:Is%20Valid
              (Effects|SpawnEmitteratLocation "/Game/Effects/Particles/P_Railgun_Impact.P_Railgun_Impact" (Transformation|GetActorLocation (Variables|/Game/SSA/Blueprints/Menues/HUD.HUD_C|GetEnemy%20Ref _ashud)))
              (Actor|DestroyActor))))))))

(event EventBeginPlay
  (Utilities|FlowControl|Delay 2.0)
  (Effects|SpawnEmitteratLocation "/Game/Effects/Particles/P_Missile_Explosion.P_Missile_Explosion" (Transformation|GetActorLocation))
  (Actor|DestroyActor))

(fn ConstructionScript)