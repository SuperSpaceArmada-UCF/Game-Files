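; Short-lived self-destruct damage actor for the Hive weapon set, centred on the player.
; On BeginPlay it moves to the player's location and destroys itself a split second later.
; Overlapping an AI-tagged actor removes enemy health through the Player, scaled by its EnemyMaxHP, and shakes the camera.
; Overlapping Debris-tagged actors instead subtracts a fixed amount from their DebrisHP.
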(event OnComponentBeginOverlap(CollisionComponent)
  (params (OtherActor :type Actor%20Object%20Reference) (OtherComp :type Primitive%20Component%20Object%20Reference) (OtherBodyIndex :type Integer) (bFromSweep :type Boolean) (SweepResult :type Hit%20Result%20Structure%20%28by%20ref%29))
  ;[1 1 1] Self Destruct Collision detection
  (if (Actor|ActorHasTag OtherActor "AI")
    (bind _asplayer (Utilities|Casting|CastToPlayer (Game|GetPlayerCharacter 0)))
    (Default|EnemyHPRemove _asplayer (/ 8.0 (Variables|/Game/SSA/Blueprints/Player_Ships/Player.Player_C|GetEnemyMaxHP _asplayer)))
    (Camera|PlayWorldCameraShake "/Game/Effects/ScreenShakeKratakosBoost.ScreenShakeKratakosBoost_C" "0, 0, 0" 0.0 1e+04)
    (elif (Actor|ActorHasTag OtherActor "Debris")
      (bind _asdebris (Utilities|Casting|CastToDebris OtherActor))
      (Variables|/Game/SSA/Blueprints/Objects/Debris.Debris_C|SetDebris%20HP _asdebris (- (Variables|/Game/SSA/Blueprints/Objects/Debris.Debris_C|GetDebris%20HP _asdebris) 1e+01)))))

(event EventBeginPlay
  ;[1 1 1] Follow Player
  (Transformation|SetActorLocation (Transformation|GetActorLocation (Game|GetPlayerCharacter 0)) false false)
  ;[1 1 1] Destroy ALL
  (Utilities|FlowControl|Delay 0.1)
  (Actor|DestroyActor))

(fn ConstructionScript)