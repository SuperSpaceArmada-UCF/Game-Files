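; Human torpedo projectile that homes on the enemy stored in the game instance and explodes on hit or after a timeout.
; Shortly after spawn it sets a homing target from that enemy's scene components, and Tick turns the mesh along its velocity.
; Hitbox overlaps reduce enemy HP through the Player for AI-tagged actors, or Debris HP directly, with explosion effects.
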(event OnComponentBeginOverlap(HitBox)
  (params (OtherActor :type Actor%20Object%20Reference) (OtherComp :type Primitive%20Component%20Object%20Reference) (OtherBodyIndex :type Integer) (bFromSweep :type Boolean) (SweepResult :type Hit%20Result%20Structure%20%28by%20ref%29))
  ;[1 1 1] Collison Enemy AI
  (if (Actor|ActorHasTag OtherActor "AI")
    (bind _asplayer (Utilities|Casting|CastToPlayer (Game|GetPlayerCharacter 0)))
    (Default|EnemyHPRemove _asplayer (/ 3.0 (Variables|/Game/SSA/Blueprints/Player_Ships/Player.Player_C|GetEnemyMaxHP _asplayer)))
    (bind _foundwidgets (Widget|GetAllWidgetsOfClass "/Game/SSA/Blueprints/Menues/HUD.HUD_C" false))
    (for _array_element _foundwidgets
      (bind _ashud (Utilities|Casting|CastToHUD _array_element))
      (Utilities|IsValid (Variables|/Game/SSA/Blueprints/Menues/HUD.HUD_C|GetEnemy%20Ref _ashud)
        (:Is%20Valid
          (Effects|SpawnEmitteratLocation "/Game/Effects/Particles/P_Missile_Explosion.P_Missile_Explosion" (Transformation|GetActorLocation (Variables|/Game/SSA/Blueprints/Menues/HUD.HUD_C|GetEnemy%20Ref _ashud)))
          (Actor|DestroyActor)
          (Camera|PlayWorldCameraShake "/Game/Effects/ScreenShakeKratakosBoost.ScreenShakeKratakosBoost_C" "0, 0, 0" 0.0 1e+04))))
    (elif (Actor|ActorHasTag OtherActor "Debris")
      (bind _asdebris (Utilities|Casting|CastToDebris OtherActor))
      (Variables|/Game/SSA/Blueprints/Objects/Debris.Debris_C|SetDebris%20HP _asdebris (- (Variables|/Game/SSA/Blueprints/Objects/Debris.Debris_C|GetDebris%20HP _asdebris) 3.0))
      (Effects|SpawnEmitteratLocation "/Game/Effects/Particles/P_Missile_Explosion.P_Missile_Explosion" (Transformation|GetActorLocation _asdebris))
      (Actor|DestroyActor))))

(event EventTick
  (params (DeltaSeconds :type Float%20%28single-precision%29))
  (bind _returnvalue (Transformation|GetActorLocation))
  ;[1 1 1] Rotator
  (Transformation|SetWorldRotation (Variables|Default|GetSkeletalMesh) (Math|Rotator|CombineRotators (Math|Rotator|FindLookatRotation _returnvalue (+ _returnvalue (Variables|/Script/Engine.MovementComponent|GetVelocity (Variables|Components|GetProjectileMovement)))) "0.000000,-90.000000,0.000000") false false))

(event EventBeginPlay
  ;[1 1 1] Homing Mechanic to AI
  (bind _asssagame_instance (Utilities|Casting|CastToSSAGameInstance (Game|GetGameInstance)))
  (Utilities|IsValid (Variables|/Game/SSA/Blueprints/SSAGameInstance.SSAGameInstance_C|GetEnemy%20Ref _asssagame_instance)
    (:Is%20Valid
      (Utilities|FlowControl|Delay 0.7)
      (for _array_element (Actor|GetComponentsByClass (Variables|/Game/SSA/Blueprints/SSAGameInstance.SSAGameInstance_C|GetEnemy%20Ref _asssagame_instance) "/Script/Engine.SceneComponent")
        (Variables|/Script/Engine.ProjectileMovementComponent|SetHomingTargetComponent (Variables|Components|GetProjectileMovement) _array_element)
        ;[1 1 1] Particle Effect
        (Utilities|FlowControl|Delay 4.0)
        (Effects|SpawnEmitteratLocation "/Game/Effects/Particles/P_Missile_Explosion.P_Missile_Explosion" (Transformation|GetActorLocation))
        (Camera|PlayWorldCameraShake "/Game/Effects/ScreenShakeKratakosBoost.ScreenShakeKratakosBoost_C" "0, 0, 0" 0.0 1e+04)
        (Actor|DestroyActor)))))

(fn ConstructionScript)