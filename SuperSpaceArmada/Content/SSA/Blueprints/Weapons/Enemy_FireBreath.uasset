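; Fire breath hazard for an enemy that damages the player while they stand inside its mesh.
; Each Tick it snaps 150 units ahead of the GameInstance's EnemyRef, matching its roll and yaw with pitch fixed at 90.
; Overlaps with "Player"-tagged actors toggle a flag, with a camera shake on entry.
; While flagged, a Delay on Tick throttles HPRemove calls to roughly half-second intervals, passing an amount divided by MaxHP.
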(event OnComponentBeginOverlap(StaticMeshComponent)
  (params (OtherActor :type Actor%20Object%20Reference) (OtherComp :type Primitive%20Component%20Object%20Reference) (OtherBodyIndex :type Integer) (bFromSweep :type Boolean) (SweepResult :type Hit%20Result%20Structure%20%28by%20ref%29))
  ;[1 1 1] Begin/End overlap
  (if (Actor|ActorHasTag OtherActor "Player")
    (Variables|Default|SetPlayer true)
    (Camera|PlayWorldCameraShake 0 "0, 0, 0" 0.0 1e+04)))

(event OnComponentEndOverlap(StaticMeshComponent)
  (params (OtherActor :type Actor%20Object%20Reference) (OtherComp :type Primitive%20Component%20Object%20Reference) (OtherBodyIndex :type Integer))
  ;[1 1 1] Begin/End overlap
  (if (Actor|ActorHasTag OtherActor "Player")
    (Variables|Default|SetPlayer false)))

(event EventTick
  (params (DeltaSeconds :type Float%20%28single-precision%29))
  (bind _asssagame_instance (Utilities|Casting|CastToSSAGameInstance (Game|GetGameInstance)))
  ;[1 1 1] Follow Player
  (Transformation|SetActorLocation (+ (Transformation|GetActorLocation (Variables|/Game/SSA/Blueprints/SSAGameInstance.SSAGameInstance_C|GetEnemy%20Ref _asssagame_instance)) (* (Transformation|GetActorForwardVector (Variables|/Game/SSA/Blueprints/SSAGameInstance.SSAGameInstance_C|GetEnemy%20Ref _asssagame_instance)) 1.5e+02)) false false)
  (Transformation|SetActorRotation (Math|Rotator|MakeRotator (.Roll (Math|Rotator|BreakRotator (Transformation|GetActorRotation (Variables|/Game/SSA/Blueprints/SSAGameInstance.SSAGameInstance_C|GetEnemy%20Ref _asssagame_instance)))) 9e+01 (.Yaw (Math|Rotator|BreakRotator (Transformation|GetActorRotation (Variables|/Game/SSA/Blueprints/SSAGameInstance.SSAGameInstance_C|GetEnemy%20Ref _asssagame_instance))))))
  ;[1 1 1] Damage Tick
  (if (Variables|Default|GetPlayer)
    (Utilities|FlowControl|Delay 0.5)
    (bind _asplayer (Utilities|Casting|CastToPlayer (Game|GetPlayerCharacter 0)))
    (Default|HPRemove _asplayer (/ 0.6 (Variables|/Game/SSA/Blueprints/Player_Ships/Player.Player_C|GetMaxHP _asplayer)))))

(fn ConstructionScript)