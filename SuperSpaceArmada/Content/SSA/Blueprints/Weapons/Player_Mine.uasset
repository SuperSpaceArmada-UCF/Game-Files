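; Player-deployed mine that arms shortly after spawning and silently destroys itself about five seconds later if not triggered.
; Sphere overlaps track AI-tagged actors, and Tick starts a half-second fuse that sets the countdown if the target has not left.
; Detonation removes enemy health through the Player character's EnemyHPRemove, scaled by EnemyMaxHP, then destroys the mine with explosion particles, camera shake and sound.
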(event OnComponentBeginOverlap(Sphere)
  (params (OtherActor :type Actor%20Object%20Reference) (OtherComp :type Primitive%20Component%20Object%20Reference) (OtherBodyIndex :type Integer) (bFromSweep :type Boolean) (SweepResult :type Hit%20Result%20Structure%20%28by%20ref%29))
  ;[1 1 1] Begin/End Overlap
  (if (Actor|ActorHasTag OtherActor "AI")
    (Variables|Default|SetAI true)
    (Variables|Default|Sethas%20left false)))

(event OnComponentEndOverlap(Sphere)
  (params (OtherActor :type Actor%20Object%20Reference) (OtherComp :type Primitive%20Component%20Object%20Reference) (OtherBodyIndex :type Integer))
  ;[1 1 1] Begin/End Overlap
  (if (Actor|ActorHasTag OtherActor "AI")
    (Variables|Default|SetAI false)
    (Variables|Default|Sethas%20left true)))

(event EventBeginPlay
  ;[1 1 1] Begin (Getting Armed)
  (Audio|SpawnSound2D "/Game/SSA/Music/Sound_Effects/Vultaari/vulta_mines.vulta_mines")
  (Utilities|FlowControl|Delay 0.25)
  (Variables|Default|SetIsReady true)
  (Utilities|FlowControl|Delay 4.75)
  (Actor|DestroyActor))

(event EventTick
  (params (DeltaSeconds :type Float%20%28single-precision%29))
  ;[1 1 1] Explosion
  (if (Variables|Default|GetIsReady)
    (if (Variables|Default|GetAI)
      (if (Variables|Default|GetCountdown)
        (bind _asplayer (Utilities|Casting|CastToPlayer (Game|GetPlayerCharacter 0)))
        (Default|EnemyHPRemove _asplayer (/ 1.0 (Variables|/Game/SSA/Blueprints/Player_Ships/Player.Player_C|GetEnemyMaxHP _asplayer)))
        (Actor|DestroyActor)
        (Effects|SpawnEmitteratLocation "/Game/Effects/Particles/P_Mine_Explosion.P_Mine_Explosion" (Transformation|GetActorLocation))
        (Camera|PlayWorldCameraShake "/Game/Effects/ScreenShakeKratakosBoost.ScreenShakeKratakosBoost_C" "0, 0, 0" 0.0 1e+04)
        (Audio|SpawnSound2D "/Game/SSA/Music/Sound_Effects/Vultaari/vult_mineHit.vult_mineHit" 2.0)
        (else
          (Utilities|FlowControl|Delay 0.5)
          (if (not (Variables|Default|Gethas%20left))
            (Variables|Default|SetCountdown true)))))))

(fn ConstructionScript)