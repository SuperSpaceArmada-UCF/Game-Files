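; Damage trigger for the player's Power Wave weapon that snaps to player character 0 every tick and hurts what overlaps it.
; Overlap events set an AI flag for AI-tagged actors and maintain an array of tagged Debris.
; Tick uses 0.1-second Delays to throttle damage, removing enemy HP through the Player blueprint, scaled by max HP, and lowering each debris piece's HP directly.
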(event OnComponentBeginOverlap(CollisionComponent)
  (params (OtherActor :type Actor%20Object%20Reference) (OtherComp :type Primitive%20Component%20Object%20Reference) (OtherBodyIndex :type Integer) (bFromSweep :type Boolean) (SweepResult :type Hit%20Result%20Structure%20%28by%20ref%29))
  ;[1 1 1] Phaser Collision detection
  (if (Actor|ActorHasTag OtherActor "AI")
    (Variables|Default|SetAI true)
    (elif (Actor|ActorHasTag OtherActor "Debris")
      (bind _asdebris (Utilities|Casting|CastToDebris OtherActor))
      (Utilities|Array|AddUnique (Variables|Default|GetDebris') _asdebris))))

(event OnComponentEndOverlap(CollisionComponent)
  (params (OtherActor :type Actor%20Object%20Reference) (OtherComp :type Primitive%20Component%20Object%20Reference) (OtherBodyIndex :type Integer))
  ;[1 1 1] Phaser Collision detection
  (if (Actor|ActorHasTag OtherActor "AI")
    (Variables|Default|SetAI false)
    (elif (Actor|ActorHasTag OtherActor "Debris")
      (bind _asdebris (Utilities|Casting|CastToDebris OtherActor))
      (Utilities|Array|RemoveItem (Variables|Default|GetDebris') _asdebris))))

(event EventTick
  (params (DeltaSeconds :type Float%20%28single-precision%29))
  ;[1 1 1] Follow Player
  (Transformation|SetActorLocation (Transformation|GetActorLocation (Game|GetPlayerCharacter 0)) false false)
  ;[1 1 1] Damage Tick
  (if (Variables|Default|GetAI)
    (Utilities|FlowControl|Delay 0.1)
    (bind _asplayer (Utilities|Casting|CastToPlayer (Game|GetPlayerCharacter 0)))
    (Default|EnemyHPRemove _asplayer (/ 0.3 (Variables|/Game/SSA/Blueprints/Player_Ships/Player.Player_C|GetEnemyMaxHP _asplayer)))
    (if (!= 0 (Utilities|Array|Length (Variables|Default|GetDebris')))
      (Utilities|FlowControl|Delay 0.1 :!label _label)
      (for _array_element (Variables|Default|GetDebris')
        (Variables|/Game/SSA/Blueprints/Objects/Debris.Debris_C|SetDebris%20HP _array_element (- (Variables|/Game/SSA/Blueprints/Objects/Debris.Debris_C|GetDebris%20HP _array_element) 0.5))))
    (elif (!= (Utilities|Array|Length (Variables|Default|GetDebris')) 0)
      (goto _label))))

(fn ConstructionScript)