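; AI_Ram_Trigger is a collision trigger that follows the AI enemy and deals ram damage on overlap.
; Each tick it searches for HUD widgets and snaps to the location of their valid EnemyRef.
; Overlapping the player removes health scaled by MaxHP, only once because the HasHurtPlayer flag is never reset here.
; Overlapping actors tagged Debris lose a fixed amount of DebrisHP.
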(event OnComponentBeginOverlap(CollisionComponent)
  (params (OtherActor :type Actor%20Object%20Reference) (OtherComp :type Primitive%20Component%20Object%20Reference) (OtherBodyIndex :type Integer) (bFromSweep :type Boolean) (SweepResult :type Hit%20Result%20Structure%20%28by%20ref%29))
  ;[1 1 1] Ram Collision detection
  (if (== OtherActor (Game|GetPlayerCharacter 0))
    (if (not (Variables|Default|GetHasHurtPlayer))
      (Variables|Default|SetHasHurtPlayer true)
      (bind _asplayer (Utilities|Casting|CastToPlayer (Game|GetPlayerCharacter 0)))
      (Default|HPRemove _asplayer (/ 4.0 (Variables|/Game/SSA/Blueprints/Player.Player_C|GetMaxHP _asplayer))))
    (elif (Actor|ActorHasTag OtherActor "Debris")
      (bind _asdebris (Utilities|Casting|CastToDebris OtherActor))
      (Variables|/Game/SSA/Blueprints/Objects/Debris.Debris_C|SetDebris%20HP _asdebris (- (Variables|/Game/SSA/Blueprints/Objects/Debris.Debris_C|GetDebris%20HP _asdebris) 7.0)))))

(event EventTick
  (params (DeltaSeconds :type Float%20%28single-precision%29))
  ;[1 1 1] Follow AI
  (bind _foundwidgets (Widget|GetAllWidgetsOfClass "/Game/SSA/Blueprints/Menues/HUD.HUD_C" false))
  (for _array_element _foundwidgets
    (bind _ashud (Utilities|Casting|CastToHUD _array_element))
    (Utilities|IsValid (Variables|/Game/SSA/Blueprints/Menues/HUD.HUD_C|GetEnemy%20Ref _ashud)
      (:Is%20Valid
        (Transformation|SetActorLocation (Transformation|GetActorLocation (Variables|/Game/SSA/Blueprints/Menues/HUD.HUD_C|GetEnemy%20Ref _ashud)) false false)))))

(fn ConstructionScript)