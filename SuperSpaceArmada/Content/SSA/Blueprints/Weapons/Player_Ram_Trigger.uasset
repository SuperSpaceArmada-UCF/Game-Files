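; Trigger actor for the player's ram attack, damaging AI enemies and debris it overlaps.
; It moves to the player character's location every Tick.
; The first AI-tagged overlap removes enemy HP through the Player's EnemyHPRemove as a fraction of max HP and plays a hit sound; HasHurtAI blocks further AI hits and is never reset here.
; Debris-tagged actors lose DebrisHP on each begin overlap.
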(event OnComponentBeginOverlap(CollisionComponent)
  (params (OtherActor :type Actor%20Object%20Reference) (OtherComp :type Primitive%20Component%20Object%20Reference) (OtherBodyIndex :type Integer) (bFromSweep :type Boolean) (SweepResult :type Hit%20Result%20Structure%20%28by%20ref%29))
  ;[1 1 1] Ram Collision detection
  (if (!= OtherActor (Game|GetPlayerCharacter 0))
    (if (Actor|ActorHasTag OtherActor "AI")
      (if (not (Variables|Default|GetHasHurtAI))
        (bind _asplayer (Utilities|Casting|CastToPlayer (Game|GetPlayerCharacter 0)))
        (Default|EnemyHPRemove _asplayer (/ 4.0 (Variables|/Game/SSA/Blueprints/Player_Ships/Player.Player_C|GetEnemyMaxHP _asplayer)))
        (Variables|Default|SetHasHurtAI true)
        (Audio|SpawnSound2D "/Game/SSA/Music/Sound_Effects/Kratokos/krata_ramHit.krata_ramHit" 2.0))
      (elif (Actor|ActorHasTag OtherActor "Debris")
        (bind _asdebris (Utilities|Casting|CastToDebris OtherActor))
        (Variables|/Game/SSA/Blueprints/Objects/Debris.Debris_C|SetDebris%20HP _asdebris (- (Variables|/Game/SSA/Blueprints/Objects/Debris.Debris_C|GetDebris%20HP _asdebris) 7.0))))))

(event EventTick
  (params (DeltaSeconds :type Float%20%28single-precision%29))
  ;[1 1 1] Follow Player
  (Transformation|SetActorLocation (Transformation|GetActorLocation (Game|GetPlayerCharacter 0)) false false))

(fn ConstructionScript)