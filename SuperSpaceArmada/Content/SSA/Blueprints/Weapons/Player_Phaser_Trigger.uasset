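; Phaser hit trigger for the player's weapon that snaps to player character 0's location every tick.
; When its collision component overlaps an actor tagged AI, it calls EnemyHPRemove on the Player with a fixed damage divided by EnemyMaxHP.
; The HasHurtAI flag limits this to one hit and is never reset here.
; The Debris tag branch does nothing, as its HP-reduction logic is disconnected.
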(event OnComponentBeginOverlap(CollisionComponent)
  (params (OtherActor :type Actor%20Object%20Reference) (OtherComp :type Primitive%20Component%20Object%20Reference) (OtherBodyIndex :type Integer) (bFromSweep :type Boolean) (SweepResult :type Hit%20Result%20Structure%20%28by%20ref%29))
  ;[1 1 1] Phaser Collision detection
  (if (!= OtherActor (Game|GetPlayerCharacter 0))
    (if (Actor|ActorHasTag OtherActor "AI")
      (if (not (Variables|Default|GetHasHurtAI))
        (bind _asplayer (Utilities|Casting|CastToPlayer (Game|GetPlayerCharacter 0)))
        (Default|EnemyHPRemove _asplayer (/ 4.0 (Variables|/Game/SSA/Blueprints/Player.Player_C|GetEnemyMaxHP _asplayer)))
        (Variables|Default|SetHasHurtAI true))
      (elif (Actor|ActorHasTag OtherActor "Debris")
        _))))

(event EventTick
  (params (DeltaSeconds :type Float%20%28single-precision%29))
  ;[1 1 1] Follow Player
  (Transformation|SetActorLocation (Transformation|GetActorLocation (Game|GetPlayerCharacter 0)) false false))

(fn ConstructionScript)