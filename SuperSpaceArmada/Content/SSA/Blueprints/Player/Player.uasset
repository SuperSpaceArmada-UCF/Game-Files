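; Player ship Blueprint for a space combat game, tracking health and energy for itself and its enemy and creating the HUD.
; A BoundaryTick timeline drives energy regeneration and a camera that frames both ships, zooming out with separation.
; Respawn events pull Human or Kratakos ships from GameInstance armadas, with player controller 0 possessing even enemy spawns.
; Boundary damage and enemy removal are empty stubs with disconnected logic.
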(event Custom|Asteroid%20Warning
  ;[1 1 1] Asteroid Belt Event
  (bind _returnvalue (UserInterface|CreateWidget "/Game/SSA/Blueprints/Menues/Asteroid_Event.Asteroid_Event_C"))
  (UserInterface|Viewport|AddtoViewport _returnvalue 0))

(event Custom|Enemy%20HP%20Restore
  (params (HP%20Plus :type Float%20%28single-precision%29))
  ;[1 1 1] Enemy HP/Energy
  (Variables|Default|SetEnemyHealth (+ HP%20Plus (Variables|Default|GetEnemyHealth))))

(event Custom|Spawn%20Next%20Ship%20Enemy
  (bind _returnvalue (Math|Random|RandomFloatinRange -1e+03 1e+03))
  (bind _returnvalue_2 (Math|Random|RandomFloatinRange -1e+03 1e+03))
  (bind _returnvalue_3 (Math|Vector|MakeVector _returnvalue_2 _returnvalue 266.0))
  (bind _returnvalue_4 (Math|Transform|MakeTransform _returnvalue_3 "0, 0, 0" "1.000000,1.000000,1.000000"))
  ;[1 1 1] Enemy Respawn
  (bind _asssagame_instance (Utilities|Casting|CastToSSAGameInstance (Game|GetGameInstance)))
  (if (> (Utilities|Array|Length (Variables|/Game/SSA/Blueprints/SSAGameInstance.SSAGameInstance_C|GetEnemy%20Armada _asssagame_instance)) 1)
    (bind _asssagame_instance_2 (Utilities|Casting|CastToSSAGameInstance (Game|GetGameInstance)))
    (Actor|DestroyActor (Variables|/Game/SSA/Blueprints/SSAGameInstance.SSAGameInstance_C|GetEnemy%20Ref _asssagame_instance_2))
    (Utilities|Array|RemoveIndex (Variables|/Game/SSA/Blueprints/SSAGameInstance.SSAGameInstance_C|GetEnemy%20Armada _asssagame_instance))
    (switch int (Utilities|Array|Get(acopy) (Variables|/Game/SSA/Blueprints/SSAGameInstance.SSAGameInstance_C|GetEnemy%20Armada _asssagame_instance)) ; SHIP TYPES:\n\n0 == Human\n1 == Kratakos
      (:Default
        (Development|PrintString "SPAWN Array OUT OF BOUNDS" true true "(R=1.000000,G=0.000000,B=0.095176,A=1.000000)" 1e+01))
      (:0
        (bind _returnvalue_5 (Game|SpawnActorfromClass "/Game/SSA/Blueprints/Player/Player_Human.Player_Human_C" _returnvalue_4 "Undefined" 0 0))
        (Pawn|Possess (Game|GetPlayerController 0) _returnvalue_5))
      (:1
        (bind _returnvalue_6 (Game|SpawnActorfromClass "/Game/SSA/Blueprints/Player/Player_Kratakos.Player_Kratakos_C" _returnvalue_4 "Undefined" 0 0))
        (Pawn|Possess (Game|GetPlayerController 0) _returnvalue_6)))
    (else
      (Utilities|Array|RemoveIndex (Variables|/Game/SSA/Blueprints/SSAGameInstance.SSAGameInstance_C|GetEnemy%20Armada _asssagame_instance)))))

(event Custom|Spawn%20Next%20Ship%20Player
  (bind _returnvalue (Math|Random|RandomFloatinRange -1e+03 1e+03))
  (bind _returnvalue_2 (Math|Random|RandomFloatinRange -1e+03 1e+03))
  (bind _returnvalue_3 (Math|Vector|MakeVector _returnvalue _returnvalue_2 266.0))
  (bind _returnvalue_4 (Math|Transform|MakeTransform _returnvalue_3 "0, 0, 0" "1.000000,1.000000,1.000000"))
  ;[1 1 1] Player Respawn
  (bind _asssagame_instance (Utilities|Casting|CastToSSAGameInstance (Game|GetGameInstance)))
  (if (> (Utilities|Array|Length (Variables|/Game/SSA/Blueprints/SSAGameInstance.SSAGameInstance_C|GetPlayer%20Armada _asssagame_instance)) 1)
    (Viewport|RemoveAllWidgets)
    (bind _outactors (Actor|GetAllActorsOfClass "Player_C"))
    (for _array_element _outactors
      (bind _asplayer (Utilities|Casting|CastToPlayer _array_element))
      (Actor|DestroyActor _asplayer)
      (Utilities|Array|RemoveIndex (Variables|/Game/SSA/Blueprints/SSAGameInstance.SSAGameInstance_C|GetPlayer%20Armada _asssagame_instance))
      (switch int (Utilities|Array|Get(acopy) (Variables|/Game/SSA/Blueprints/SSAGameInstance.SSAGameInstance_C|GetPlayer%20Armada _asssagame_instance)) ; SHIP TYPES:\n\n0 == Human\n1 == Kratakos
        (:Default
          (Development|PrintString "SPAWN Array OUT OF BOUNDS" true true "(R=1.000000,G=0.000000,B=0.095176,A=1.000000)" 1e+01))
        (:0
          (bind _returnvalue_5 (Game|SpawnActorfromClass "/Game/SSA/Blueprints/Player/Player_Human.Player_Human_C" _returnvalue_4 "Undefined" 0 0))
          (Pawn|Possess (Game|GetPlayerController 0) _returnvalue_5))
        (:1
          (bind _returnvalue_6 (Game|SpawnActorfromClass "/Game/SSA/Blueprints/Player/Player_Kratakos.Player_Kratakos_C" _returnvalue_4 "Undefined" 0 0))
          (Pawn|Possess (Game|GetPlayerController 0) _returnvalue_6))))
    (else
      (Utilities|Array|RemoveIndex (Variables|/Game/SSA/Blueprints/SSAGameInstance.SSAGameInstance_C|GetPlayer%20Armada _asssagame_instance)))))

(event Custom|Enemy%20HP%20Remove
  (params (HP%20Minus :type Float%20%28single-precision%29))
  ;[1 1 1] Enemy HP/Energy
  (if (not (Variables|Default|GetEnemy%20IsImmortal))
    (bind _output_get (Variables|Default|SetEnemyHealth (- (Variables|Default|GetEnemyHealth) HP%20Minus)))
    (if (<= _output_get 0.0)
      (CallFunction|EnemyRemove))))

(event Custom|Remove%20Asteroid%20Warning
  ;[1 1 1] Asteroid Belt Event
  (Widget|RemovefromParent (stale Custom|Asteroid%20Warning _returnvalue)))

(event Custom|HP%20Remove
  (params (HP%20Minus :type Float%20%28single-precision%29))
  ;[1 1 1] HP/Energy
  (if (not (Variables|Default|GetIsImmortal))
    (Variables|Default|SetHealth (- (Variables|Default|GetHealth) HP%20Minus))))

(event Custom|HP%20Restore
  (params (HP%20Plus :type Float%20%28single-precision%29))
  ;[1 1 1] HP/Energy
  (Variables|Default|SetHealth (+ HP%20Plus (Variables|Default|GetHealth))))

(event Custom|Energy%20Remove
  (params (Energy%20Minus :type Float%20%28single-precision%29))
  ;[1 1 1] HP/Energy
  (Variables|Default|SetEnergy (- (Variables|Default|GetEnergy) Energy%20Minus)))

(event Custom|Energy%20Restore
  (params (Energy%20Plus :type Float%20%28single-precision%29))
  ;[1 1 1] HP/Energy
  (Variables|Default|SetEnergy (+ Energy%20Plus (Variables|Default|GetEnergy))))

(event Custom|Enemy%20Energy%20Restore
  (params (Energy%20Plus :type Float%20%28single-precision%29))
  ;[1 1 1] Enemy HP/Energy
  (Variables|Default|SetEnemyEnergy (+ Energy%20Plus (Variables|Default|GetEnemyEnergy))))

(event Custom|Enemy%20Energy%20Remove
  (params (Energy%20Minus :type Float%20%28single-precision%29))
  ;[1 1 1] Enemy HP/Energy
  (Variables|Default|SetEnemyEnergy (- (Variables|Default|GetEnemyEnergy) Energy%20Minus)))

(event EventBeginPlay
  ;[1 1 1] Begin
  (bind _returnvalue (UserInterface|CreateWidget "/Game/SSA/Blueprints/Menues/HUD.HUD_C"))
  (bind _output_get (Variables|Default|SetHUD%20Reference _returnvalue))
  (UserInterface|Viewport|AddtoViewport _output_get 0)
  (Variables|/Game/SSA/Blueprints/Menues/HUD.HUD_C|SetMy%20Character _returnvalue self)
  (Input|SetInputModeGameOnly (Game|GetPlayerController 0))
  (Timeline|Boundary%20Tick PlayFromStart
    (:Update
      (CallFunction|CameraMove)
      (CallFunction|BoundaryDamage)
      (Utilities|FlowControl|Delay 1.0)
      (CallFunction|EnergyRestore (/ 1.0 (Variables|Default|GetMaxEnergy))))))

(event Input|KeyboardEvents|F
  (params (Key :type Key%20Structure :default "AnyKey"))
  ;[1 1 1] To Be Deleted
)

(fn ConstructionScript)

(fn EnemyRemove)

(fn LoadEnemies
  (params (Input%20Array :type Array%20of%20Actor%20Object%20References))
  ;[1 1 1] Array of Enemies (0 is on field) called from level BP
  (Variables|Default|SetEnemy%20Array Input%20Array))

(fn InitializeShip
  (bind _giref (LocalVariables|GetGIRef))
  (Variables|Default|SetHealth (Utilities|Array|Get(acopy) (Variables|/Game/SSA/Blueprints/SSAGameInstance.SSAGameInstance_C|GetHealthArray _giref)))
  (Variables|Default|SetEnergy (Utilities|Array|Get(acopy) (Variables|/Game/SSA/Blueprints/SSAGameInstance.SSAGameInstance_C|GetEnergyArray _giref)))
  (Variables|/Script/Engine.CharacterMovementComponent|SetMaxFlySpeed (Variables|Character|GetCharacterMovement) (Utilities|Array|Get(acopy) (Variables|/Game/SSA/Blueprints/SSAGameInstance.SSAGameInstance_C|GetSpeedArray _giref)))
  (Components|StaticMesh|SetStaticMesh (Variables|Default|GetHuman_Mesh) 0))

(fn CameraMove
  (bind _returnvalue (Transformation|GetActorLocation))
  (bind _enemy (Variables|Default|GetEnemy))
  (bind _returnvalue_2 (Transformation|GetActorLocation _enemy))
  (bind _returnvalue_3 (- _returnvalue_2 _returnvalue))
  (bind (_x _y) (Math|Vector|BreakVector _returnvalue_3))
  (if (Utilities|IsValid _enemy)
    (if (not (Game|IsGamePaused))
      (LocalVariables|SetMid%20point (+ (/ _returnvalue_3 2) _returnvalue))
      (Transformation|SetWorldLocation (Variables|Default|GetCamera1) (Math|Vector|MakeVector (.X (Math|Vector|BreakVector (+ (/ (- _returnvalue (LocalVariables|GetMid%20point)) 2) (LocalVariables|GetMid%20point)))) (.Y (Math|Vector|BreakVector (+ (/ (- _returnvalue (LocalVariables|GetMid%20point)) 2) (LocalVariables|GetMid%20point)))) (+ (/ (+ (Math|Float|Absolute(Float) _x) (Math|Float|Absolute(Float) _y)) 2.0) 1e+03)) false false))))

(fn SetEnemyRef
  ;[1 1 1] Called by the HUD to set enemy Ref
  (bind _foundwidgets (Widget|GetAllWidgetsOfClass "/Game/SSA/Blueprints/Menues/HUD.HUD_C" false))
  (for _array_element _foundwidgets
    (bind _ashud (Utilities|Casting|CastToHUD _array_element))
    (bind _output_get (Variables|Default|SetEnemy (Variables|/Game/SSA/Blueprints/Menues/HUD.HUD_C|GetEnemy%20Ref _ashud)))
    (Development|PrintString (Utilities|String|ToString(Vector) (Transformation|GetActorLocation _output_get)))))

(fn BoundaryDamage
  ;[1 1 1] Boundary Tick
)