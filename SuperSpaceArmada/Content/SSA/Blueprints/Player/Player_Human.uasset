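; Human player ship for SSA, extending a parent player class with normalised health and energy and registering itself with the game instance.
; Left click fires a torpedo with sound and cooldown; right click spawns a phaser trigger and starts a recursive, delayed loop draining energy.
; F subtracts health, spawning the next ship at zero.
; Arena boundary damage and one phaser stop sequence are disconnected, so never run.
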(event Custom|Phasers
  ;[1 1 1] Human Secondary
  (if (Variables|Default|GetPressed)
    (if (Utilities|IsValid (Variables|Default|GetSecondaryAtk))
      (if (Audio|Components|Audio|IsPlaying (Variables|Default|GetSecondaryAtk))
        _
        (else
          (bind _returnvalue (Audio|SpawnSound2D "/Game/SSA/Music/Sound_Effects/Phasers.Phasers" :!label _label))
          (bind _output_get (Variables|Default|SetSecondaryAtk _returnvalue))
          (Audio|Components|Audio|Play _output_get 0.0)))
      (else
        (goto _label)))
    (if (>= (Variables|Default|GetEnergy) (/ 3.0 (Variables|Default|GetMaxEnergy)))
      (Utilities|FlowControl|Delay 1.0)
      (CallFunction|EnergyRemove (/ 3.0 (Variables|Default|GetMaxEnergy)))
      (CallFunction|Phasers)
      (else
        (Variables|Default|SetPressed false)))
    (else
      (Actor|DestroyActor (stale Input|MouseEvents|RightMouseButton _returnvalue))
      (Utilities|IsValid (Variables|Default|GetSecondaryAtk)
        (:Is%20Valid
          (Audio|Components|Audio|Stop (Variables|Default|GetSecondaryAtk)))))))

(event EventTick
  (params (DeltaSeconds :type Float%20%28single-precision%29))
  ;[1 1 1] Boundary Tick
)

(event EventBeginPlay
  ;[1 1 1] Human Construct
  (bind _asssagame_instance (Utilities|Casting|CastToSSAGameInstance (Game|GetGameInstance)))
  (Variables|/Game/SSA/Blueprints/SSAGameInstance.SSAGameInstance_C|SetPlayer%20Ref _asssagame_instance self)
  (Variables|Default|SetMaxHP 14.0)
  (Variables|Default|SetHealth 1.0)
  (Variables|Default|SetMaxEnergy 1e+01)
  (Variables|Default|SetEnergy 1.0)
  (|CallParentFunction))

(event Input|MouseEvents|RightMouseButton
  (params (Key :type Key%20Structure :default "AnyKey"))
  ;[1 1 1] Human Secondary
  (:Pressed
    (if (>= (Variables|Default|GetEnergy) 0.1)
      (Variables|Default|SetPressed true)
      (CallFunction|EnergyRemove (/ 1.0 (Variables|Default|GetMaxEnergy)))
      (bind _returnvalue (Game|SpawnActorfromClass "/Game/SSA/Blueprints/Weapons/Player_Phaser_Trigger.Player_Phaser_Trigger_C" (Transformation|GetActorTransform) "Undefined" 0 0))
      (AddComponent|AddChildActorComponent _returnvalue false)
      (CallFunction|Phasers))))

(event Input|MouseEvents|LeftMouseButton
  (params (Key :type Key%20Structure :default "AnyKey"))
  (bind _returnvalue (Transformation|GetActorRotation))
  ;[1 1 1] Human Primary
  (:Pressed
    (if (Variables|Default|GetPrimaryWeaponCD)
      (if (>= (Variables|Default|GetEnergy) 0.2)
        (Variables|Default|SetPrimaryWeaponCD false)
        (bind _returnvalue_2 (Audio|SpawnSound2D "/Game/SSA/Music/Sound_Effects/Laser_Cue.Laser_Cue"))
        (Audio|Components|Audio|Play _returnvalue_2 0.0)
        (Game|SpawnActorfromClass "/Game/SSA/Blueprints/Weapons/Human_Torpedo.Human_Torpedo_C" (Math|Transform|MakeTransform (+ (* (Math|Vector|GetForwardVector _returnvalue) 4.2e+02) (Transformation|GetActorLocation)) _returnvalue) "Undefined" 0 0)
        (CallFunction|EnergyRemove (/ 2.0 (Variables|Default|GetMaxEnergy)))
        (Utilities|FlowControl|Delay 3.0)
        (Variables|Default|SetPrimaryWeaponCD true)))))

(event Input|KeyboardEvents|F
  (params (Key :type Key%20Structure :default "AnyKey"))
  (:Pressed
    (bind _output_get (Variables|Default|SetHealth (- (Variables|Default|GetHealth) 0.5)))
    (if (<= _output_get 0.0)
      (CallFunction|SpawnNextShipPlayer))))

(fn ConstructionScript
  (|CallParentFunction))

(fn BoundaryDam)