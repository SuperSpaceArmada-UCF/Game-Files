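; Debris collider actor that damages whatever it hits and then destroys itself.
; The Hit event passes the other actor to DebrisCollisionFunc, which applies a fixed amount of damage to it before destroying the debris.
; An unconnected node for spawning a Bullet ahead of the actor remains in the graph and never runs.
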(event EventBeginPlay)

(event EventActorBeginOverlap
  (params (OtherActor :type Actor%20Object%20Reference)))

(event Collision|EventHit
  (params (MyComp :type Primitive%20Component%20Object%20Reference) (Other :type Actor%20Object%20Reference) (OtherComp :type Primitive%20Component%20Object%20Reference) (bSelfMoved :type Boolean) (HitLocation :type Vector :default "0, 0, 0") (HitNormal :type Vector :default "0, 0, 0") (NormalImpulse :type Vector :default "0, 0, 0") (Hit :type Hit%20Result%20Structure%20%28by%20ref%29))
  (CallFunction|DebrisCollisionFunc Other))

(event EventTick
  (params (DeltaSeconds :type Float%20%28single-precision%29)))

(fn ConstructionScript)

(fn DebrisCollisionFunc
  (params (Collider :type Actor%20Object%20Reference))
  (Game|Damage|ApplyDamage Collider 1e+02 0 0)
  (Actor|DestroyActor))